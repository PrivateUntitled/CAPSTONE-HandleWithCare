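; Level 1 narrative sequencer that sets the objective, shows the title and, unless pack onboarding is done, runs the packing tutorial after the title card fades.
; Chained delegates and timers advance one reusable checklist widget through spawning a box, placing items, packing away and Q item detection.
; It gates steps by toggling package spawning, box buttons and Visibility-channel collision on the package and exit door, which is restored at the end.
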(event `self.ReceiveBeginPlay`
  (bind _titlecardwidget (`/Game/Blueprints/GameModes/BP_GM_Main.TitleCardWidget` (`self.As BP GM Main`)))
  (`parent.ReceiveBeginPlay`)
  (bind _asbp_third_person_character (cast `/Game/ThirdPerson/Blueprints/BP_ThirdPersonCharacter` (`GameplayStatics.GetPlayerPawn` 0)))
  (set `self.As BP Third Person Character` _asbp_third_person_character)
  (set `/Game/GameInstance/BP_GameInstance.CurrentObjective` (`self.TargetObjectiveAfter`) (`self.As BP Game Instance`))
  (set `/Game/GameInstance/BP_GameInstance.UnpackOnboardDone` true (`self.As BP Game Instance`))
  (bind _returnvalue (`GameplayStatics.GetActorOfClass` "/Game/Blueprints/Furniture/Doors/BP_A_ExitDoor.BP_A_ExitDoor_C"))
  (`PrimitiveComponent.SetCollisionResponseToChannel` (`/Game/Blueprints/Furniture/Doors/BP_A_ExitDoor.StaticMesh` _returnvalue) "ECC_Visibility" "ECR_Ignore")
  (`self.ShowTitle`)
  (if (not (`/Game/GameInstance/BP_GameInstance.PackOnboardDone` (`self.As BP Game Instance`)))
    (`UserWidget.BindToAnimationFinished` _titlecardwidget (`/Game/Blueprints/Widgets/WB_TitleCard.FadeOut` _titlecardwidget) (delegate `CustomEvent_0`))))

(event `CustomEvent_0`
  (`/Game/Blueprints/GameModes/BP_GM_Main.GetAllItems` (`self.As BP GM Main`))
  (`/Game/Blueprints/Narrative/AC_Narrative.AddDialogue` (`self.AC_Narrative`) "/Game/Blueprints/Narrative/DataAssets/Level1/DA_DG_Level1_Intro.DA_DG_Level1_Intro")
  (bind _returnvalue (`|CreateWidget` "/Game/Blueprints/Widgets/WB_ReusableWidget.WB_ReusableWidget_C"))
  (bind _output_get (set `self.TutorialWidget` _returnvalue))
  (`UserWidget.AddToViewport` _output_get 0)
  (`/Game/Blueprints/Widgets/WB_ReusableWidget.SetText` (`self.TutorialWidget`) "Press E on the Package Zone to Spawn Box" true)
  (add `/Game/Blueprints/PackingBlueprints/BP_PackageZone.PackageSpawned` (`self.PackageZone`) (delegate `CustomEvent`)))

(event `CustomEvent`
  (bind _packagezone (`self.PackageZone`))
  (`self.CheckBox` true)
  (remove `/Game/Blueprints/PackingBlueprints/BP_PackageZone.PackageSpawned` _packagezone (delegate `CustomEvent`))
  (`KismetSystemLibrary.Delay` 0.0001)
  (set `/Game/Blueprints/PackingBlueprints/BP_PackageZone.CanSpawnPackages?` false _packagezone)
  (if (== (`self.SequenceIdx`) 0)
    (set `self.SequenceIdx` 1)
    (bind _returnvalue (`GameplayStatics.GetActorOfClass` "/Game/Blueprints/Box/BP_A_Package.BP_A_Package_C"))
    (`PrimitiveComponent.SetCollisionResponseToChannel` (`/Game/Blueprints/ItemInteractables/BP_A_ItemInteractable.Collision` _returnvalue) "ECC_Visibility" "ECR_Ignore")
    (`KismetSystemLibrary.K2_SetTimerDelegate` (delegate `Delay1`) 4.0)))

(event `Delay1`
  (bind _returnvalue (`GameplayStatics.GetActorOfClass` "/Game/Blueprints/Box/BP_A_Package.BP_A_Package_C"))
  (`PrimitiveComponent.SetCollisionResponseToChannel` (`/Game/Blueprints/ItemInteractables/BP_A_ItemInteractable.Collision` _returnvalue) "ECC_Visibility" "ECR_Block")
  (`/Game/Blueprints/Widgets/WB_ReusableWidget.SetText` (`self.TutorialWidget`) "Look around the house and place the items in the box." false)
  (add `/Game/Blueprints/Box/BP_A_Package.OnOpenPackage` _returnvalue (delegate `CheckIfItemIsValid`)))

(event `CheckBox`
  (params (isCheck :type Boolean))
  (`/Game/Blueprints/Widgets/WB_ReusableWidget.ChangeCheckBox` (`self.TutorialWidget`) isCheck))

(event `CheckIfItemIsValid`
  (bind _currentbox (`/Game/ThirdPerson/Blueprints/BP_ThirdPersonCharacter.CurrentBox` (`self.As BP Third Person Character`)))
  (bind _boxwidget (`/Game/Blueprints/Box/BP_A_Package.BoxWidget` _currentbox))
  (bind _backbutton (`/Game/Blueprints/Player/PlayerUI/WB_BoxUI.BackButton` _boxwidget))
  (bind _packawaybutton (`/Game/Blueprints/Player/PlayerUI/WB_BoxUI.PackAwayButton` _boxwidget))
  (`KismetSystemLibrary.Delay` 0.2)
  (if (`KismetArrayLibrary.Array_IsValidIndex` (`/Game/Blueprints/Box/BP_A_Package.OutBox` (`/Game/ThirdPerson/Blueprints/BP_ThirdPersonCharacter.CurrentBox` (`self.As BP Third Person Character`))))
    (remove `/Game/Blueprints/Box/BP_A_Package.OnOpenPackage` _currentbox (delegate `CheckIfItemIsValid`))
    (set `Widget.Visibility` "Hidden" _backbutton)
    (`Widget.SetIsEnabled` _backbutton false)
    (set `Widget.Visibility` "Hidden" _packawaybutton)
    (`Widget.SetIsEnabled` _packawaybutton false)
    (`/Game/Blueprints/Widgets/WB_ReusableWidget.SetText` (`self.TutorialWidget`) "Place the item in the box" true)
    (for _array_element (`/Game/Blueprints/Box/BP_A_Package.OutBox` (`/Game/ThirdPerson/Blueprints/BP_ThirdPersonCharacter.CurrentBox` (`self.As BP Third Person Character`)))
      (add `/Game/Blueprints/ItemInteractables/BP_A_ItemInteractable.ItemInGrid` _array_element (delegate `PackAwayOnboard`)))))

(event `PackAwayOnboard`
  (`self.CheckBox` true)
  (for _array_element (`/Game/Blueprints/Box/BP_A_Package.OutBox` (`/Game/ThirdPerson/Blueprints/BP_ThirdPersonCharacter.CurrentBox` (`self.As BP Third Person Character`)))
    (remove `/Game/Blueprints/ItemInteractables/BP_A_ItemInteractable.ItemInGrid` _array_element (delegate `PackAwayOnboard`)))
  (for _array_element_2 (`/Game/Blueprints/Box/BP_A_Package.InBox` (`/Game/ThirdPerson/Blueprints/BP_ThirdPersonCharacter.CurrentBox` (`self.As BP Third Person Character`)))
    (remove `/Game/Blueprints/ItemInteractables/BP_A_ItemInteractable.ItemInGrid` _array_element_2 (delegate `PackAwayOnboard`)))
  (`KismetSystemLibrary.K2_SetTimerDelegate` (delegate `Delay2`) 4.0))

(event `Delay2`
  (bind _packawaybutton (`/Game/Blueprints/Player/PlayerUI/WB_BoxUI.PackAwayButton` (`/Game/Blueprints/Box/BP_A_Package.BoxWidget` (`/Game/ThirdPerson/Blueprints/BP_ThirdPersonCharacter.CurrentBox` (`self.As BP Third Person Character`)))))
  (set `Widget.Visibility` "Visible" _packawaybutton)
  (`Widget.SetIsEnabled` _packawaybutton true)
  (`/Game/Blueprints/Widgets/WB_ReusableWidget.SetText` (`self.TutorialWidget`) "Once done filling up the box you can click the \"Pack Away\" button to store it" true)
  (add `/Game/Blueprints/Box/BP_A_Package.Stored` (`/Game/ThirdPerson/Blueprints/BP_ThirdPersonCharacter.CurrentBox` (`self.As BP Third Person Character`)) (delegate `NextSeq`)))

(event `NextSeq`
  (`self.CheckBox` true)
  (`KismetSystemLibrary.K2_SetTimerDelegate` (delegate `Delay3`) 4.0))

(event `Delay3`
  (set `/Game/Blueprints/PackingBlueprints/BP_PackageZone.CanSpawnPackages?` true (`self.PackageZone`))
  (`/Game/Blueprints/Widgets/WB_ReusableWidget.SetText` (`self.TutorialWidget`) "If you need more boxes, you can always spawn more." false)
  (add `/Game/Blueprints/PackingBlueprints/BP_PackageZone.PackageSpawned` (`self.PackageZone`) (delegate `QOnboard`)))

(event `QOnboard`
  (remove `/Game/Blueprints/PackingBlueprints/BP_PackageZone.PackageSpawned` (`self.PackageZone`) (delegate `QOnboard`))
  (`/Game/Blueprints/Widgets/WB_ReusableWidget.SetText` (`self.TutorialWidget`) "You can press \"Q\" to detect all the items in the level!" true)
  (add `/Game/ThirdPerson/Blueprints/BP_ThirdPersonCharacter.QPressed` (`self.As BP Third Person Character`) (delegate `QPressed`)))

(event `QPressed`
  (`self.CheckBox` true)
  (`KismetSystemLibrary.K2_SetTimerDelegate` (delegate `CustomEvent_5`) 5.0))

(event `CustomEvent_5`
  (`/Game/Blueprints/Widgets/WB_ReusableWidget.SetText` (`self.TutorialWidget`) "When you are done, just approach the door and leave." true)
  (`KismetSystemLibrary.K2_SetTimerDelegate` (delegate `CustomEvent_7`) 5.0))

(event `CustomEvent_7`
  (bind _returnvalue (`GameplayStatics.GetActorOfClass` "/Game/Blueprints/Furniture/Doors/BP_A_ExitDoor.BP_A_ExitDoor_C"))
  (`PrimitiveComponent.SetCollisionResponseToChannel` (`/Game/Blueprints/Furniture/Doors/BP_A_ExitDoor.StaticMesh` _returnvalue) "ECC_Visibility" "ECR_Block")
  (set `/Game/GameInstance/BP_GameInstance.UnpackOnboardDone` true (`self.As BP Game Instance`))
  (`Widget.RemoveFromParent` (`self.TutorialWidget`)))

(fn `UserConstructionScript`
  (`parent.UserConstructionScript`))