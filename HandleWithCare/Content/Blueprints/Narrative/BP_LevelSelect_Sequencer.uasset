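; Narrative sequencer for the level-select map that plays dialogue based on the Game Instance's current objective.
; On BeginPlay it restores the truck's last saved location, then starts the intro or a level or ending dialogue.
; The intro chains timers and delays: dialogue with input disabled, a camera blend to the office building and back, then timed tutorial text.
; StartSequenceToOffice plays Level 1 end dialogue but is not called here.
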(event `self.ReceiveBeginPlay`
  (bind _as_bp_truck_ls (`self.As BP Truck LS`))
  (bind _currentobjective (`/Game/GameInstance/BP_GameInstance.CurrentObjective` (`self.As BP Game Instance`)))
  (bind _asbp_truck_ls (cast `/Game/Blueprints/CarMovement/BP_TruckLS` (`GameplayStatics.GetPlayerPawn` 0)))
  (set `self.As BP Truck LS` _asbp_truck_ls)
  (bind _asbp_game_instance (cast `/Game/GameInstance/BP_GameInstance` (`GameplayStatics.GetGameInstance`)))
  (bind _output_get (set `self.As BP Game Instance` _asbp_game_instance))
  (bind _locationstruct (`/Game/GameInstance/BP_GameInstance.LocationStruct` _output_get))
  (if (!= (.location (break `/Game/GameInstance/Structures/LocationData` _locationstruct)) (0.0 0.0 0.0))
    (`self.K2_SetActorLocation` (`self.As BP Truck LS`) (.location (break `/Game/GameInstance/Structures/LocationData` _locationstruct)) false false))
  (`|ExecutionSequence`
    (:`then_0`
      (if (`|EnumEquality` _currentobjective "NewEnumerator8")
        (`SceneComponent.SetHiddenInGame` (`/Game/Blueprints/CarMovement/BP_TruckLS.arrow1` _as_bp_truck_ls) true false)
        (`/Game/Blueprints/CarMovement/BP_TruckLS.StartMoving` _as_bp_truck_ls)
        (`self.StartIntroSequence`)))
    (:`then_1`
      (if (`|EnumEquality` _currentobjective "NewEnumerator10")
        (`self.StartSequenceToLevel1`)))
    (:`then_2`
      (if (`|EnumEquality` _currentobjective "NewEnumerator6")
        (`self.StartSequenceToLevel2A`)))
    (:`then_3`
      (if (`|EnumEquality` _currentobjective "NewEnumerator12")
        (`self.StartSequenceToEnding`)))))

(event `StartIntroSequence`
  (bind _ac_narrative (`self.AC_Narrative`))
  (bind _as_bp_truck_ls (`self.As BP Truck LS`))
  (`self.DisableInput` _as_bp_truck_ls (`/Game/Blueprints/CarMovement/BP_TruckLS.As BP Player Controller` _as_bp_truck_ls))
  (`/Game/Blueprints/Narrative/AC_Narrative.AddDialogue` _ac_narrative "/Game/Blueprints/Narrative/DataAssets/LevelSelect/LevelSelect_Intro/DA_DG_LevelSelect_Intro1.DA_DG_LevelSelect_Intro1")
  (`KismetSystemLibrary.K2_SetTimerDelegate` (delegate `ShowBuilding`) (`/Game/Blueprints/Narrative/WB_Narrative.TotalTime` (`/Game/Blueprints/Narrative/AC_Narrative.Narrative` _ac_narrative))))

(event `ShowBuilding`
  (bind _as_bp_truck_ls (`self.As BP Truck LS`))
  (bind _as_bp_truck_ls_2 (`self.As BP Truck LS`))
  (bind _as_bp_player_controller (`/Game/Blueprints/CarMovement/BP_TruckLS.As BP Player Controller` _as_bp_truck_ls))
  (`SceneComponent.SetHiddenInGame` (`/Game/Blueprints/CarMovement/BP_TruckLS.arrow1` _as_bp_truck_ls_2) false false)
  (set `/Game/Blueprints/CarMovement/BP_TruckLS.Stop` true _as_bp_truck_ls_2)
  (bind _returnvalue (`GameplayStatics.GetActorOfClass` "/Game/Blueprints/LevelSelect/Actors/BP_OfficeBuilding.BP_OfficeBuilding_C"))
  (`PlayerController.SetViewTargetWithBlend` _as_bp_player_controller _returnvalue 3.0 "VTBlend_Linear" 0.0 false)
  (`KismetSystemLibrary.Delay` 5.0)
  (`self.EnableInput` _as_bp_truck_ls _as_bp_player_controller)
  (`PlayerController.SetViewTargetWithBlend` _as_bp_player_controller _as_bp_truck_ls 1.0 "VTBlend_Linear" 0.0 false)
  (`KismetSystemLibrary.Delay` 1.0)
  (`/Game/Blueprints/Narrative/AC_Narrative.AddDialogue` (`self.AC_Narrative`) "/Game/Blueprints/Narrative/DataAssets/LevelSelect/LevelSelect_Intro/DA_DG_LevelSelect_Intro2.DA_DG_LevelSelect_Intro2")
  (bind _returnvalue_2 (`|GenericCreateObject` "/Game/Blueprints/Widgets/WB_TutorialWidget.WB_TutorialWidget_C"))
  (`UserWidget.AddToViewport` _returnvalue_2 0)
  (`KismetSystemLibrary.K2_SetTimerDelegate` (delegate `NextSequence`) 5.0))

(event `NextSequence`
  (set `TextBlock.Text` "Follow the arrow to reach your destination" (`/Game/Blueprints/Widgets/WB_TutorialWidget.TextBlock_25` (stale `ShowBuilding` _returnvalue_2)))
  (`KismetSystemLibrary.K2_SetTimerDelegate` (delegate `NextSequence2`) 7.0))

(event `StartSequenceToLevel1`
  (`/Game/Blueprints/Narrative/AC_Narrative.AddDialogue` (`self.AC_Narrative`) "/Game/Blueprints/Narrative/DataAssets/LevelSelect/LevelSelect_Level1/DA_DG_LevelSelect_Level1_Intro.DA_DG_LevelSelect_Level1_Intro"))

(event `NextSequence2`
  (`Widget.RemoveFromParent` (stale `ShowBuilding` _returnvalue_2)))

(event `StartSequenceToOffice`
  (`/Game/Blueprints/Narrative/AC_Narrative.AddDialogue` (`self.AC_Narrative`) "/Game/Blueprints/Narrative/DataAssets/LevelSelect/LevelSelect_Level1/DA_DG_LevelSelect_Level1_End.DA_DG_LevelSelect_Level1_End"))

(event `StartSequenceToLevel2A`
  (`/Game/Blueprints/Narrative/AC_Narrative.AddDialogue` (`self.AC_Narrative`) "/Game/Blueprints/Narrative/DataAssets/LevelSelect/LevelSelect_Level2A/DA_DG_LevelSelect_Level2A_Intro.DA_DG_LevelSelect_Level2A_Intro"))

(event `StartSequenceToEnding`
  (`/Game/Blueprints/Narrative/AC_Narrative.AddDialogue` (`self.AC_Narrative`) "/Game/Blueprints/Narrative/DataAssets/LevelSelect/LevelSelect_Level3/DA_DG_LevelSelect_Level3_Intro.DA_DG_LevelSelect_Level3_Intro"))

(fn `UserConstructionScript`
  (`parent.UserConstructionScript`))