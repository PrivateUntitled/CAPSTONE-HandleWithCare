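; Narrative sequencer for Level 3 that sets the game instance's objective, quest and onboarding state and turns off packing mode on BeginPlay.
; It respawns saved Level 0 items at their stored transforms, setting them and, beforehand, existing furniture to ignore WorldStatic collision.
; It then shows the title card, whose fade-out triggers item gathering and the second intro dialogue.
; The first intro dialogue and its timed StartLevel call are disconnected.
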(event `self.ReceiveBeginPlay`
  (bind _as_bp_game_instance (`self.As BP Game Instance`))
  (bind _titlecardwidget (`/Game/Blueprints/GameModes/BP_GM_Main.TitleCardWidget` (`self.As BP GM Main`)))
  (`parent.ReceiveBeginPlay`)
  (set `/Game/GameInstance/BP_GameInstance.CurrentObjective` "NewEnumerator12" _as_bp_game_instance)
  (set `/Game/GameInstance/BP_GameInstance.CurrentQuest` "/Game/UI/Widgets/Mail/Data/DA_ClientMail4.DA_ClientMail4" _as_bp_game_instance)
  (set `/Game/GameInstance/BP_GameInstance.UnpackOnboardDone` true _as_bp_game_instance)
  (set `/Game/Blueprints/GameModes/BP_GM_Main.isPacking` false (`self.As BP GM Main`))
  (`self.GetLevel0Items`)
  (`self.ShowTitle` :!label _label)
  (`UserWidget.BindToAnimationFinished` _titlecardwidget (`/Game/Blueprints/Widgets/WB_TitleCard.FadeOut` _titlecardwidget) (delegate `Done`)))

(event `StartLevel`
  (goto _label))

(event `Done`
  (`/Game/Blueprints/GameModes/BP_GM_Main.GetAllItems` (`self.As BP GM Main`))
  (`/Game/Blueprints/Narrative/AC_Narrative.AddDialogue` (`self.AC_Narrative`) "/Game/Blueprints/Narrative/DataAssets/Level3/DA_DG_Level3_Intro2.DA_DG_Level3_Intro2"))

(fn `GetLevel0Items`
  (bind _level0items (`/Game/GameInstance/BP_GameInstance.Level0Items` (`self.As BP Game Instance`)))
  (if (`KismetArrayLibrary.Array_IsNotEmpty` _level0items)
    (bind _outactors (`GameplayStatics.GetAllActorsOfClass` "/Game/Blueprints/Furniture/BP_A_Furniture.BP_A_Furniture_C"))
    (for _array_element _outactors
      (`PrimitiveComponent.SetCollisionResponseToChannel` (`/Game/Blueprints/Furniture/BP_A_Furniture.BoxCollision` _array_element) "ECC_WorldStatic" "ECR_Ignore"))
    (for _array_element_2 _level0items
      (bind _returnvalue (`|SpawnActorFromClass` (break `/Game/Blueprints/Structure/ItemStruct` _array_element_2) (`KismetMathLibrary.MakeTransform` (`.Location_6_E6A949BB445CB969F790878C051740C6` (break `/Game/Blueprints/Structure/ItemStruct` _array_element_2)) (`.Rotation_9_F1B159DE4DBA65746B89F99085B07607` (break `/Game/Blueprints/Structure/ItemStruct` _array_element_2))) "Undefined" "MultiplyWithRoot" null null))
      (`PrimitiveComponent.SetCollisionResponseToChannel` (`/Game/Blueprints/ItemInteractables/BP_A_ItemInteractable.Collision` _returnvalue) "ECC_WorldStatic" "ECR_Ignore"))))

(fn `UserConstructionScript`
  (`parent.UserConstructionScript`))