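; Level 2B narrative sequencer that runs the opening of the level, from loading screen to intro dialogue.
; BeginPlay shows a loading screen, whose completion event removes it, resumes music, sets the objective and client-mail quest, clears packing mode and marks onboarding steps done.
; It then shows the title card and, when its fade-out finishes, calls GetAllItems on the game mode and queues the intro dialogue.
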(event `DoneLoading`
  (bind _as_bp_game_instance (`self.As BP Game Instance`))
  (bind _as_bp_game_instance_2 (`self.As BP Game Instance`))
  (bind _titlecardwidget (`/Game/Blueprints/GameModes/BP_GM_Main.TitleCardWidget` (`self.As BP GM Main`)))
  (`Widget.RemoveFromParent` (stale `self.ReceiveBeginPlay` _returnvalue))
  (`AudioComponent.SetPaused` (`/Game/Blueprints/GameModes/BP_GM_Main.CurrentBGM` (`self.As BP GM Main`)) false)
  (set `/Game/GameInstance/BP_GameInstance.CurrentObjective` (`self.TargetObjectiveAfter`) _as_bp_game_instance_2)
  (set `/Game/GameInstance/BP_GameInstance.CurrentQuest` "/Game/UI/Widgets/Mail/Data/DA_ClientMail3.DA_ClientMail3" _as_bp_game_instance_2)
  (set `/Game/Blueprints/GameModes/BP_GM_Main.isPacking` false (`self.As BP GM Main`))
  (set `/Game/GameInstance/BP_GameInstance.UnpackOnboardDone` true _as_bp_game_instance)
  (set `/Game/GameInstance/BP_GameInstance.PackOnboardDone` true _as_bp_game_instance)
  (set `/Game/GameInstance/BP_GameInstance.EmailOnboardDone` true _as_bp_game_instance)
  (`self.ShowTitle`)
  (`UserWidget.BindToAnimationFinished` _titlecardwidget (`/Game/Blueprints/Widgets/WB_TitleCard.FadeOut` _titlecardwidget) (delegate `Done`)))

(event `self.ReceiveBeginPlay`
  (`parent.ReceiveBeginPlay`)
  (bind _returnvalue (`|GenericCreateObject` "/Game/Blueprints/Widgets/WB_LoadingScreen.WB_LoadingScreen_C"))
  (`UserWidget.AddToViewport` _returnvalue 0)
  (add `/Game/Blueprints/Widgets/WB_LoadingScreen.DoneLoading` _returnvalue (delegate `DoneLoading`)))

(event `Done`
  (`/Game/Blueprints/GameModes/BP_GM_Main.GetAllItems` (`self.As BP GM Main`))
  (`/Game/Blueprints/Narrative/AC_Narrative.AddDialogue` (`self.AC_Narrative`) "/Game/Blueprints/Narrative/DataAssets/Level2B/DA_DG_Level2B_Intro.DA_DG_Level2B_Intro"))

(fn `UserConstructionScript`
  (`parent.UserConstructionScript`))