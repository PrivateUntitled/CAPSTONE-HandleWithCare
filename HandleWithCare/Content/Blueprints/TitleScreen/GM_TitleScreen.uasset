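; Game mode for the title screen that shows the menu widget and resets the game instance's session state.
; BeginPlay creates BP_TitleScreen, sets mouse-driven game-and-UI input, and runs console commands for screen messages and a frame-rate cap.
; SetGameInstance restores starting quest, objective, onboarding flags and player upgrades, clears packages and items, and rewrites each client star entry's existing name.
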(event `self.ReceiveBeginPlay`
  (bind _returnvalue (`GameplayStatics.GetPlayerController` 0))
  (`KismetSystemLibrary.ExecuteConsoleCommand` "EnableAllScreenMessages" null)
  (`KismetSystemLibrary.ExecuteConsoleCommand` "t.MaxFPS 144" null)
  (bind _returnvalue_2 (`|GenericCreateObject` "/Game/UI/Widgets/BP_TitleScreen.BP_TitleScreen_C"))
  (`UserWidget.AddToViewport` _returnvalue_2 0)
  (bind _asbp_game_instance (cast `/Game/GameInstance/BP_GameInstance` (`GameplayStatics.GetGameInstance`)))
  (set `self.As BP Game Instance` _asbp_game_instance)
  (`self.SetGameInstance`)
  (set `PlayerController.bShowMouseCursor` true _returnvalue)
  (`WidgetBlueprintLibrary.SetInputMode_GameAndUIEx` _returnvalue null "DoNotLock" false))

(fn `SetGameInstance`
  (bind _as_bp_game_instance (`self.As BP Game Instance`))
  (bind _clientstardata (`/Game/GameInstance/BP_GameInstance.ClientStarData` _as_bp_game_instance))
  (set `/Game/GameInstance/BP_GameInstance.CurrentObjective` "NewEnumerator8" _as_bp_game_instance)
  (`KismetArrayLibrary.Array_Clear` (`/Game/GameInstance/BP_GameInstance.Packages` _as_bp_game_instance))
  (set `/Game/GameInstance/BP_GameInstance.CurrentQuest` "/Game/UI/Widgets/Mail/Data/DA_ClientMail0.DA_ClientMail0" _as_bp_game_instance)
  (`KismetArrayLibrary.Array_Clear` (`/Game/GameInstance/BP_GameInstance.Level0Items` _as_bp_game_instance))
  (set `/Game/GameInstance/BP_GameInstance.UnpackOnboardDone` false _as_bp_game_instance)
  (set `/Game/GameInstance/BP_GameInstance.PackOnboardDone` false _as_bp_game_instance)
  (set `/Game/GameInstance/BP_GameInstance.EmailOnboardDone` false _as_bp_game_instance)
  (set `/Game/GameInstance/BP_GameInstance.LocationStruct` (make `/Game/GameInstance/Structures/LocationData` "0.000000,0.000000,0.000000|0.000000,0.000000,0.000000|1.000000,1.000000,1.000000") _as_bp_game_instance)
  (set `/Game/GameInstance/BP_GameInstance.QuestTaskIndex` 0 _as_bp_game_instance)
  (for (_array_element _array_index) _clientstardata
    (setmembers `/Game/GameInstance/Structures/ClientData` :`StructRef` (`|GetArrayItem` _clientstardata _array_index) :`ClientName` (break `/Game/GameInstance/Structures/ClientData` _array_element) :`Stars` 0 :`HasReplied` false))
  (set `/Game/GameInstance/BP_GameInstance.isInOptionsTitleScreen` true _as_bp_game_instance)
  (set `/Game/GameInstance/BP_GameInstance.TutorialSkip` false _as_bp_game_instance)
  (set `/Game/GameInstance/BP_GameInstance.PlayerUpgrades` (make `/Game/GameInstance/Upgrades/UpgradeList` (make `/Game/GameInstance/Upgrades/UpgradeLevels` "/Game/GameInstance/Upgrades/DA_MoveSpeed.DA_MoveSpeed") (make `/Game/GameInstance/Upgrades/UpgradeLevels` "/Game/GameInstance/Upgrades/DA_MaxWeightItem.DA_MaxWeightItem") (make `/Game/GameInstance/Upgrades/UpgradeLevels` "/Game/GameInstance/Upgrades/DA_BoxSize.DA_BoxSize") (make `/Game/GameInstance/Upgrades/UpgradeLevels` "/Game/GameInstance/Upgrades/DA_BoxAmtUpgrade.DA_BoxAmtUpgrade")) _as_bp_game_instance))

(fn `UserConstructionScript`)