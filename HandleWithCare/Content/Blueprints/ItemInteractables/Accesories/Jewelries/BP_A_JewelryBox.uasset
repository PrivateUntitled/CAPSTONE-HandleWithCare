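; BP_A_JewelryBox is an interactable jewelry box accessory with an animated lid.
; On BeginPlay it registers the Cover mesh with its StaticMeshes list and binds opening to the item-in-grid event and closing to the item-detached event.
; Two timelines lerp the Cover's roll between closed and open angles.
; An IsOpen flag, updated when each timeline finishes, gates both actions, and each finish stops the opposite timeline.
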(event `self.ReceiveBeginPlay`
  (`parent.ReceiveBeginPlay`)
  (`KismetArrayLibrary.Array_AddUnique` (`self.StaticMeshes`) (`self.Cover`))
  (add `self.ItemInGrid` (delegate `Open`))
  (add `self.ItemDetached` (delegate `Close`)))

(event `Open`
  (if (not (`self.isOpen`))
    (bind (_direction _openfloat) (`Timeline|OpenLid T` :!via `PlayFromStart` :!label _label)
      (:`Update`
        (`SceneComponent.K2_SetRelativeRotation` (`self.Cover`) (`KismetMathLibrary.MakeRotator` (`KismetMathLibrary.Lerp` (`self.LidClose`) (`self.LidOpen`) _openfloat)) false false))
      (:`Finished`
        (set `self.isOpen` true)
        (bind (_direction_2 _closefloat) (`Timeline|CloseLid T` :!via `Stop` :!label _label_2)
          (:`Update`
            (`SceneComponent.K2_SetRelativeRotation` (`self.Cover`) (`KismetMathLibrary.MakeRotator` (`KismetMathLibrary.Lerp` (`self.LidOpen`) (`self.LidClose`) _closefloat)) false false))
          (:`Finished`
            (set `self.isOpen` false)
            (goto _label :!via `Stop`)))))))

(event `Close`
  (if (`self.isOpen`)
    (goto _label_2 :!via `PlayFromStart`)))

(fn `UserConstructionScript`
  (`parent.UserConstructionScript`))