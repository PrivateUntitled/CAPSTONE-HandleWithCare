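; BP_A_Books is an office book item that randomizes its materials on BeginPlay and can trigger an achievement based on how it is placed.
; It binds CheckBookKieller to an item-in-grid event.
; Outside packing mode, that check awards DA_Achievement_SP_BK when the character's current furniture is a bookshelf, IsForward is set, and the book's right vector points along the shelf's local negative X.
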(event `self.ReceiveBeginPlay`
  (`parent.ReceiveBeginPlay`)
  (add `self.ItemInGrid` (delegate `CheckBookKieller`))
  (`self.RandomizeMats` 0))

(event `CheckBookKieller`
  (bind _currentfurniture (`/Game/ThirdPerson/Blueprints/BP_ThirdPersonCharacter.CurrentFurniture` (`self.As BP Third Person Character`)))
  (bind _asbp_gm_main (cast `/Game/Blueprints/GameModes/BP_GM_Main` (`GameplayStatics.GetGameMode`)))
  (if (`/Game/Blueprints/GameModes/BP_GM_Main.isPacking` _asbp_gm_main)
    _
    (elif (== (`GameplayStatics.GetObjectClass` _currentfurniture) "/Game/Blueprints/Furniture/BP_A_Bookshelves.BP_A_Bookshelves_C")
      (if (`self.isForward`)
        (if (== (`KismetMathLibrary.BreakVector3f` (`KismetMathLibrary.InverseTransformDirection` (`self.GetTransform` _currentfurniture) (`self.GetActorRightVector`))) -1.0)
          (`/Game/Blueprints/Achievements/AC_Achievements.Display Achievement` (`/Game/ThirdPerson/Blueprints/BP_ThirdPersonCharacter.AC_Achievements` (`self.As BP Third Person Character`)) "/Game/Blueprints/Achievements/Achievements_DataAssets/SP/DA_Achievement_SP_BK.DA_Achievement_SP_BK"))))))

(fn `UserConstructionScript`
  (`parent.UserConstructionScript`))