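; Folded clothes item that gives itself a random look when play begins.
; After the parent BeginPlay, it picks a random index from SwitchedMaterialList and passes it to RandomizeMaterials.
; That function applies the entry's folded material to the static mesh and stores its matching unfolded materials in SwitchedStaticMeshMaterial, keeping both states paired.
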(event `self.ReceiveBeginPlay`
  (`parent.ReceiveBeginPlay`)
  (`self.RandomizeMaterials` (`.OutIndex` (`KismetArrayLibrary.Array_Random` (`self.SwitchedMaterialList`)))))

(fn `RandomizeMaterials`
  (params (`Random Int` :type Integer))
  (bind (_foldedmaterial _unfoldedmaterials) (break `/Game/Blueprints/ItemInteractables/Clothes/ClothesMaterialStruct` (`|GetArrayItem` (`self.SwitchedMaterialList`) `Random Int`)))
  (if (`KismetArrayLibrary.Array_IsValidIndex` (`self.SwitchedMaterialList`))
    (set `self.SwitchedStaticMeshMaterial` _unfoldedmaterials)
    (`PrimitiveComponent.SetMaterial` (`self.StaticMesh`) 0 _foldedmaterial)))

(fn `UserConstructionScript`
  (`parent.UserConstructionScript`))