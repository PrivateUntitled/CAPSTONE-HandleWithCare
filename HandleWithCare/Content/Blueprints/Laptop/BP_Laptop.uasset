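; Interactable laptop actor that opens a paused in-game browser UI with links to mail and upgrade screens.
; Cursor hover enables E input and custom-depth highlighting, with interaction gated by onboarding, current quest and a held-item check.
; Each screen clears all widgets, shows a new one and binds its navigation events, while a tutorial index sequences perks then email hints.
; Exiting unpauses and restores the player UI and roaming controls.
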(event `ShowMailPanel`
  (bind _widget (`self.Widget`))
  (`WidgetLayoutLibrary.RemoveAllWidgets`)
  (bind _returnvalue (`|CreateWidget` "/Game/UI/Widgets/BP_Mail.BP_Mail_C"))
  (`UserWidget.AddToViewport` _returnvalue 0)
  (`WidgetComponent.SetWidget` _widget _returnvalue)
  (bind _asbp_mail (cast `/Game/UI/Widgets/BP_Mail` (`WidgetComponent.GetWidget` _widget)))
  (add `/Game/UI/Widgets/BP_Mail.ExitMail` _asbp_mail (`|CreateDelegate` :!event `EnterMainBrowser`)))

(event `ShowUpgradePanel`
  (bind _widget (`self.Widget`))
  (`WidgetLayoutLibrary.RemoveAllWidgets`)
  (bind _returnvalue (`|CreateWidget` "/Game/UI/Widgets/WB_Upgrades.WB_Upgrades_C"))
  (`UserWidget.AddToViewport` _returnvalue 0)
  (`WidgetComponent.SetWidget` _widget _returnvalue)
  (bind _aswb_upgrades (cast `/Game/UI/Widgets/WB_Upgrades` (`WidgetComponent.GetWidget` _widget)))
  (add `/Game/UI/Widgets/WB_Upgrades.ExitUpgrades` _aswb_upgrades (`|CreateDelegate` :!event `EnterMainBrowser`))
  (if (and (not (`/Game/GameInstance/BP_GameInstance.EmailOnboardDone` (`self.As BP Game Instance`))) (== (`self.LaptopTutorialIndex`) 0))
    (`/Engine/EditorBlueprintResources/StandardMacros.IncrementInt` (`self.LaptopTutorialIndex`))))

(event `EnterMainBrowser`
  (bind _widget (`self.Widget`))
  (`WidgetLayoutLibrary.RemoveAllWidgets`)
  (bind _returnvalue (`|CreateWidget` "/Game/UI/Widgets/WB_MainBrowser.WB_MainBrowser_C"))
  (`UserWidget.AddToViewport` _returnvalue 0)
  (`WidgetComponent.SetWidget` _widget _returnvalue)
  (bind _aswb_main_browser (cast `/Game/UI/Widgets/WB_MainBrowser` (`WidgetComponent.GetWidget` _widget)))
  (add `/Game/UI/Widgets/WB_MainBrowser.ExitLaptop` _aswb_main_browser (`|CreateDelegate` :!event `ExitLaptop`))
  (add `/Game/UI/Widgets/WB_MainBrowser.EnterEmail` _aswb_main_browser (`|CreateDelegate` :!event `ShowMailPanel`))
  (add `/Game/UI/Widgets/WB_MainBrowser.EnterUpgrades` _aswb_main_browser (`|CreateDelegate` :!event `ShowUpgradePanel`))
  (if (not (`/Game/GameInstance/BP_GameInstance.EmailOnboardDone` (`self.As BP Game Instance`)))
    (switch `int` (`self.LaptopTutorialIndex`)
      (:`0`
        (`/Game/UI/Widgets/WB_MainBrowser.PerksTutorials` _aswb_main_browser))
      (:`1`
        (`/Game/UI/Widgets/WB_MainBrowser.EmailTutorial` _aswb_main_browser)))))

(event `self.Box.OnBeginCursorOver`
  (params (TouchedComponent :type "PrimitiveComponent Object Reference"))
  (bind _as_bp_third_person_character (`self.As BP Third Person Character`))
  ;[0.4554 0.2597 0.7396] Enable Interact (E) when cursor on the truck
  (`/Engine/EditorBlueprintResources/StandardMacros.IsValid` (`self.As BP Third Person Character`)
    (:`Is Valid`
      (if (not (`/Game/ThirdPerson/Blueprints/BP_ThirdPersonCharacter.IsInteracting` (`self.As BP Third Person Character`)))
        (set `/Game/ThirdPerson/Blueprints/BP_ThirdPersonCharacter.Laptop` self _as_bp_third_person_character)
        (`self.EnableInput` (`/Game/ThirdPerson/Blueprints/BP_ThirdPersonCharacter.As BP Player Controller` _as_bp_third_person_character))
        (`KismetSystemLibrary.PrintString` "Hello")
        (bind _asbp_game_instance (cast `/Game/GameInstance/BP_GameInstance` (`GameplayStatics.GetGameInstance`)))
        (if (`/Game/GameInstance/BP_GameInstance.UnpackOnboardDone` _asbp_game_instance)
          (if (not (== (`/Game/GameInstance/BP_GameInstance.CurrentQuest` (`self.As BP Game Instance`)) "/Game/UI/Widgets/Mail/Data/DA_ClientMail4.DA_ClientMail4"))
            (set `/Game/ThirdPerson/Blueprints/BP_ThirdPersonCharacter.HasHoveredItem` true _as_bp_third_person_character)
            (`PrimitiveComponent.SetRenderCustomDepth` (`self.StaticMesh`) true)))))))

(event `self.ReceiveBeginPlay`
  (bind _asbp_third_person_character (cast `/Game/ThirdPerson/Blueprints/BP_ThirdPersonCharacter` (`GameplayStatics.GetPlayerPawn` 0)))
  (set `self.As BP Third Person Character` _asbp_third_person_character)
  (bind _asbp_player_controller (cast `/Game/Blueprints/Player/BP_PlayerController` (`GameplayStatics.GetPlayerController` 0)))
  (set `self.As BP Player Controller` _asbp_player_controller)
  (bind _asbp_game_instance (cast `/Game/GameInstance/BP_GameInstance` (`GameplayStatics.GetGameInstance`)))
  (set `self.As BP Game Instance` _asbp_game_instance))

(event `Key|E`
  (params (Key :type "Key Structure"))
  (bind _marker (`self.Marker`))
  (bind _as_bp_third_person_character (`self.As BP Third Person Character`))
  (:`Pressed`
    (bind _asbp_game_instance (cast `/Game/GameInstance/BP_GameInstance` (`GameplayStatics.GetGameInstance`)))
    (if (`/Game/GameInstance/BP_GameInstance.UnpackOnboardDone` _asbp_game_instance)
      (if (not (== (`/Game/GameInstance/BP_GameInstance.CurrentQuest` _asbp_game_instance) "/Game/UI/Widgets/Mail/Data/DA_ClientMail4.DA_ClientMail4"))
        (`/Engine/EditorBlueprintResources/StandardMacros.IsValid` _as_bp_third_person_character
          (:`Is Valid`
            (if (not (`KismetSystemLibrary.DoesImplementInterface` (`|GetArrayItem` (`/Game/ThirdPerson/Blueprints/BP_ThirdPersonCharacter.Items` _as_bp_third_person_character) 1)))
              (`GameplayStatics.SetGamePaused` true)
              (set `/Game/ThirdPerson/Blueprints/BP_ThirdPersonCharacter.IsInteracting` true (`self.As BP Third Person Character`))
              (`/Game/Blueprints/Player/BP_PlayerController.SetMouse` (`self.As BP Player Controller`) false true)
              (`self.EnterMainBrowser`)
              (if (not (`SceneComponent.bHiddenInGame` _marker))
                (`SceneComponent.SetHiddenInGame` _marker true false)))))))))

(event `self.Box.OnEndCursorOver`
  (params (TouchedComponent :type "PrimitiveComponent Object Reference"))
  (bind _as_bp_third_person_character (`self.As BP Third Person Character`))
  (bind _as_bp_third_person_character_2 (`self.As BP Third Person Character`))
  ;[0.4554 0.2597 0.7396] Disable Interact (E) when cursor off the truck
  (`/Engine/EditorBlueprintResources/StandardMacros.IsValid` (`self.As BP Third Person Character`)
    (:`Is Valid`
      (if (not (`/Game/ThirdPerson/Blueprints/BP_ThirdPersonCharacter.IsInteracting` _as_bp_third_person_character_2))
        (set `/Game/ThirdPerson/Blueprints/BP_ThirdPersonCharacter.Laptop` null _as_bp_third_person_character_2)
        (`self.DisableInput` (`/Game/ThirdPerson/Blueprints/BP_ThirdPersonCharacter.As BP Player Controller` _as_bp_third_person_character))
        (bind _asbp_game_instance (cast `/Game/GameInstance/BP_GameInstance` (`GameplayStatics.GetGameInstance`)))
        (if (`/Game/GameInstance/BP_GameInstance.UnpackOnboardDone` _asbp_game_instance)
          (set `/Game/ThirdPerson/Blueprints/BP_ThirdPersonCharacter.HasHoveredItem` false _as_bp_third_person_character)
          (`PrimitiveComponent.SetRenderCustomDepth` (`self.StaticMesh`) false))))))

(event `ExitLaptop`
  (bind _as_bp_player_controller (`self.As BP Player Controller`))
  (`GameplayStatics.SetGamePaused` false)
  (set `/Game/Blueprints/Player/BP_PlayerController.Roaming` true _as_bp_player_controller)
  (set `PlayerController.bShowMouseCursor` false _as_bp_player_controller)
  (set `/Game/ThirdPerson/Blueprints/BP_ThirdPersonCharacter.IsInteracting` false (`self.As BP Third Person Character`))
  (`WidgetLayoutLibrary.RemoveAllWidgets`)
  (bind _returnvalue (`|GenericCreateObject` "/Game/Blueprints/Player/PlayerUI/WB_PlayerUI.WB_PlayerUI_C"))
  (`UserWidget.AddToViewport` _returnvalue 0)
  (`/Game/Blueprints/Player/BP_PlayerController.SetMouse` (`self.As BP Player Controller`) true false))

(fn `UserConstructionScript`)