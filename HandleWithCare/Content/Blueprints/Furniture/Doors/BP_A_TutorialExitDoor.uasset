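; Tutorial exit door actor that gates leaving the level on its completion percentage.
; On BeginPlay it runs the parent logic, then sets its static mesh to ignore the Visibility collision channel.
; Pressing E checks the main game mode's completion value, showing the exit door widget if incomplete or the result screen widget at full completion.
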(event `self.ReceiveBeginPlay`
  (`parent.ReceiveBeginPlay`)
  (`PrimitiveComponent.SetCollisionResponseToChannel` (`self.StaticMesh`) "ECC_Visibility" "ECR_Ignore"))

(event `Key|E`
  (params (Key :type "Key Structure"))
  (:`Pressed`
    (if (!= (`/Game/Blueprints/GameModes/BP_GM_Main.LevelCompletionPercentage` (`self.As BP GM Main`)) 1.0)
      (`UserWidget.AddToViewport` (`self.ExitDoorWidget`) 0)
      (else
        (`UserWidget.AddToViewport` (`/Game/Blueprints/GameModes/BP_GM_Main.ResultScreenWidget` (`self.As BP GM Main`)) 0)))))

(fn `UserConstructionScript`
  (`parent.UserConstructionScript`))