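; Wall furniture Blueprint that highlights its mesh when hovered or opened, extending a parent furniture class.
; Hover applies a red highlight material, and unhover restores a transparent one and clears the character's hovered-furniture state, both only while the character is not interacting.
; Opening always applies the red highlight after the parent logic, while closing and construction just defer to the parent.
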(event `self.On Hover`
  (`parent.On Hover`)
  (if (not (`/Game/ThirdPerson/Blueprints/BP_ThirdPersonCharacter.IsInteracting` (`self.As BP Third Person Character`)))
    (`PrimitiveComponent.SetMaterial` (`self.StaticMesh`) 0 "/Game/Blueprints/Materials/HighlightRed.HighlightRed")))

(event `self.OnUnhover`
  (bind _as_bp_third_person_character (`self.As BP Third Person Character`))
  (if (not (`/Game/ThirdPerson/Blueprints/BP_ThirdPersonCharacter.IsInteracting` _as_bp_third_person_character))
    (set `/Game/ThirdPerson/Blueprints/BP_ThirdPersonCharacter.CurrentHoveredFurniture` null _as_bp_third_person_character)
    (set `/Game/ThirdPerson/Blueprints/BP_ThirdPersonCharacter.HasHoveredItem` false _as_bp_third_person_character)
    (`PrimitiveComponent.SetMaterial` (`self.StaticMesh`) 0 "/Game/Blueprints/Materials/Transparent2.Transparent2")))

(event `self.OpenFurniture`
  (`parent.OpenFurniture`)
  (`PrimitiveComponent.SetMaterial` (`self.StaticMesh`) 0 "/Game/Blueprints/Materials/HighlightRed.HighlightRed"))

(event `self.OnFurnitureClose`
  (`parent.OnFurnitureClose`))

(fn `UserConstructionScript`
  (`parent.UserConstructionScript`))