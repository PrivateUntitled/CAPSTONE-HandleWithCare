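; Wall picture furniture actor that spawns its switchable picture parts from BP_A_WallPictures in the construction script.
; On BeginPlay it collects each part's static mesh and applies its mesh state with a basic wall material.
; On unhover it clears the character's hovered furniture and restores original materials, except that meshless parts after the first mesh entry turn highlight red.
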(event `self.ReceiveBeginPlay`
  (`parent.ReceiveBeginPlay`)
  (for _array_element (`self.FurniturePartsChild`)
    (bind _asbp_a_switchable_items (cast `/Game/Blueprints/Furniture/FurnitureParts/SwitchableItems/BP_A_SwitchableItems` _array_element))
    (`KismetArrayLibrary.Array_Add` (`self.StaticMeshes`) (`/Game/Blueprints/Furniture/FurnitureParts/SwitchableItems/BP_A_SwitchableItems.StaticMesh` _asbp_a_switchable_items))
    (`/Game/Blueprints/Furniture/FurnitureParts/SwitchableItems/BP_A_SwitchableItems.SwitchMesh` _asbp_a_switchable_items (`self.hasMesh`) null "/Game/StarterContent/Materials/M_Basic_Wall.M_Basic_Wall")))

(event `self.OnUnhover`
  (bind _as_bp_third_person_character (`self.As BP Third Person Character`))
  (set `/Game/ThirdPerson/Blueprints/BP_ThirdPersonCharacter.CurrentHoveredFurniture` null _as_bp_third_person_character)
  (set `/Game/ThirdPerson/Blueprints/BP_ThirdPersonCharacter.HasHoveredItem` false _as_bp_third_person_character)
  (for (_array_element _array_index) (`self.StaticMeshes`)
    (if (!= _array_index 0)
      (bind _asbp_a_switchable_items (cast `/Game/Blueprints/Furniture/FurnitureParts/SwitchableItems/BP_A_SwitchableItems` (`ActorComponent.GetOwner` _array_element)))
      (if (`/Game/Blueprints/Furniture/FurnitureParts/SwitchableItems/BP_A_SwitchableItems.hasMesh` _asbp_a_switchable_items)
        (`PrimitiveComponent.SetMaterial` _array_element 0 (`self.OriginalMaterial`))
        (else
          (for (_ _array_index_2) (`MeshComponent.GetMaterials` _array_element)
            (`PrimitiveComponent.SetMaterial` _array_element _array_index_2 "/Game/Blueprints/Materials/HighlightRed.HighlightRed"))))
      (else
        (`PrimitiveComponent.SetMaterial` _array_element 0 (`self.OriginalMaterial`))))))

(fn `UserConstructionScript`
  (`parent.UserConstructionScript`)
  (`self.SpawnFurnitureParts` (`self.WallPictures`) "/Game/Blueprints/Furniture/FurnitureParts/SwitchableItems/BP_A_WallPictures.BP_A_WallPictures_C"))