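; Wall furniture Blueprint for a toilet wall that carries toilet holder parts.
; The construction script spawns BP_A_ToiletHolder parts through SpawnFurnitureParts on ToiletWall and stores them in Child.
; BeginPlay gathers each child's Holder mesh into StaticMeshes without duplicates, then passes the children, HasMesh and the RandomItem class to CheckHasMesh.
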(event `self.ReceiveBeginPlay`
  (`parent.ReceiveBeginPlay`)
  (for _array_element (`self.Child`)
    (bind _asbp_a_toilet_holder (cast `/Game/Blueprints/Furniture/FurnitureParts/SwitchableItems/BP_A_ToiletHolder` _array_element))
    (`KismetArrayLibrary.Array_AddUnique` (`self.StaticMeshes`) (`/Game/Blueprints/Furniture/FurnitureParts/SwitchableItems/BP_A_ToiletHolder.Holder` _asbp_a_toilet_holder)))
  (`self.CheckHasMesh` (`self.hasMesh`) (`self.RandomItem`) (`self.Child`)))

(fn `UserConstructionScript`
  (`parent.UserConstructionScript`)
  (bind _child (`self.SpawnFurnitureParts` (`self.ToiletWall`) "/Game/Blueprints/Furniture/FurnitureParts/SwitchableItems/BP_A_ToiletHolder.BP_A_ToiletHolder_C"))
  (set `self.Child` _child))