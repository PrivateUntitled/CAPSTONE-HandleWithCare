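; Cabinet furniture actor with three child drawers and slot grids on both the cabinet and each drawer.
; The construction script spawns BP_A_Drawer parts and builds a 3x3 grid on the cabinet plus a 2x2 grid per drawer.
; BeginPlay gathers the grids and drawer meshes into arrays.
; Opening the cabinet disables collision on drawer grid boxes, leaving the cabinet grid untouched, and closing it shuts any open drawers.
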(event `self.ReceiveBeginPlay`
  (bind _gridstruct (`self.GridStruct`))
  (`parent.ReceiveBeginPlay`)
  (`KismetArrayLibrary.Array_Add` _gridstruct (make `/Game/Blueprints/Structure/GridStruct` (`self.Grids`)))
  (`KismetArrayLibrary.Array_Add` _gridstruct (make `/Game/Blueprints/Structure/GridStruct` (`self.Grids2`)))
  (`KismetArrayLibrary.Array_Add` _gridstruct (make `/Game/Blueprints/Structure/GridStruct` (`self.Grids3`)))
  (`KismetArrayLibrary.Array_Add` _gridstruct (make `/Game/Blueprints/Structure/GridStruct` (`self.Grids4`)))
  (for _array_element (`self.FurniturePartsChild`)
    (bind _asbp_a_drawer (cast `/Game/Blueprints/Furniture/FurnitureParts/BP_A_Drawer` _array_element))
    (`KismetArrayLibrary.Array_Add` (`self.StaticMeshes`) (`/Game/Blueprints/Furniture/FurnitureParts/BP_A_Drawer.StaticMesh` _asbp_a_drawer))))

(event `self.OnFurnitureOpen`
  (`parent.OnFurnitureOpen`)
  (for _array_element (`self.GridStruct`)
    (if (not (`KismetArrayLibrary.Array_Identical` (`self.Grids4`) (break `/Game/Blueprints/Structure/GridStruct` _array_element)))
      (for _array_element_2 (break `/Game/Blueprints/Structure/GridStruct` _array_element)
        (`PrimitiveComponent.SetCollisionEnabled` (`/Game/Blueprints/Box/Grids/BP_A_Grid.Box` _array_element_2) "NoCollision")))))

(event `self.OnFurnitureClose`
  (`parent.OnFurnitureClose`)
  (for _array_element (`self.FurniturePartsChild`)
    (bind _asbp_a_drawer (cast `/Game/Blueprints/Furniture/FurnitureParts/BP_A_Drawer` _array_element))
    (if (`/Game/Blueprints/Furniture/FurnitureParts/BP_A_Drawer.isOpen` _asbp_a_drawer)
      (`/Game/Blueprints/Furniture/FurnitureParts/BP_A_Drawer.Close` _asbp_a_drawer))))

(fn `UserConstructionScript`
  (`parent.UserConstructionScript`)
  (`self.InitializeGrid` 3 3 (`self.GridTest`) (`self.Grids4`) 10.0)
  (`self.SpawnFurnitureParts` (`self.CabinetDrawers`) "/Game/Blueprints/Furniture/FurnitureParts/BP_A_Drawer.BP_A_Drawer_C")
  (bind _asbp_a_drawer (cast `/Game/Blueprints/Furniture/FurnitureParts/BP_A_Drawer` (`|GetArrayItem` (`self.FurniturePartsChild`))))
  (`self.InitializeGrid` 2 2 (`/Game/Blueprints/Furniture/FurnitureParts/BP_A_Drawer.GridPosition` _asbp_a_drawer) (`self.Grids`))
  (bind _asbp_a_drawer_2 (cast `/Game/Blueprints/Furniture/FurnitureParts/BP_A_Drawer` (`|GetArrayItem` (`self.FurniturePartsChild`) 1)))
  (`self.InitializeGrid` 2 2 (`/Game/Blueprints/Furniture/FurnitureParts/BP_A_Drawer.GridPosition` _asbp_a_drawer_2) (`self.Grids2`))
  (bind _asbp_a_drawer_3 (cast `/Game/Blueprints/Furniture/FurnitureParts/BP_A_Drawer` (`|GetArrayItem` (`self.FurniturePartsChild`) 2)))
  (`self.InitializeGrid` 2 2 (`/Game/Blueprints/Furniture/FurnitureParts/BP_A_Drawer.GridPosition` _asbp_a_drawer_3) (`self.Grids3`)))