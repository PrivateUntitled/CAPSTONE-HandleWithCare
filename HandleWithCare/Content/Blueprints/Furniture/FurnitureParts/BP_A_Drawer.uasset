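; Clickable furniture drawer that slides open and closed when its owner is the player's current furniture, highlighting on hover while closed.
; Open and Close toggle attached grid collision and fire dispatchers that drive two timelines lerping its relative location.
; Opening closes any open sibling drawers in the owning cabinet.
; When each slide finishes, the cabinet's InItems switch Visibility collision to Block or Ignore.
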(event `self.ReceiveBeginPlay`
  (bind _returnvalue_location (`KismetMathLibrary.BreakTransform` (`SceneComponent.GetRelativeTransform` (`self.DefaultSceneRoot`))))
  (bind _returnvalue (`SceneComponent.GetRelativeTransform` (`self.DefaultSceneRoot`)))
  (bind _asbp_third_person_character (cast `/Game/ThirdPerson/Blueprints/BP_ThirdPersonCharacter` (`GameplayStatics.GetPlayerPawn` 0)))
  (set `self.As BP Third Person Character` _asbp_third_person_character)
  (set `self.OriginalLocation` _returnvalue_location)
  (set `self.EndLocation` (`KismetMathLibrary.MakeVector` (+ (.x (.location _returnvalue)) 25.0) (.y (.location _returnvalue)) (.z (.location _returnvalue))))
  (add `self.Opened` (delegate `OpenDrawer`))
  (add `self.Closed` (delegate `CloseDrawer`)))

(event `CloseDrawer`
  (bind (_direction _opendrawer) (`Timeline|Timeline_0` :!via `PlayFromStart` :!label _label)
    (:`Update`
      (`self.K2_SetActorRelativeLocation` self (`KismetMathLibrary.VLerp` (`self.EndLocation`) (`self.OriginalLocation`) _opendrawer) false false)
      (bind (_direction_2 _opendrawer_2) (`Timeline|Timeline` :!via `Stop` :!label _label_2)
        (:`Update`
          (`self.K2_SetActorRelativeLocation` self (`KismetMathLibrary.VLerp` (`self.OriginalLocation`) (`self.EndLocation`) _opendrawer_2) false false)
          (goto _label :!via `Stop`))
        (:`Finished`
          (bind _asbp_a_cabinet_drawer (cast `/Game/Blueprints/Furniture/BP_A_CabinetDrawer` (`self.GetOwner`)))
          (bind _initems (`/Game/Blueprints/Furniture/BP_A_Furniture.InItems` _asbp_a_cabinet_drawer))
          (if (`KismetArrayLibrary.Array_IsValidIndex` _initems)
            (for _array_element _initems
              (`PrimitiveComponent.SetCollisionResponseToChannel` (`/Game/Blueprints/ItemInteractables/BP_A_ItemInteractable.Collision` _array_element) "ECC_Visibility" "ECR_Block"))))))
    (:`Finished`
      (bind _asbp_a_cabinet_drawer_2 (cast `/Game/Blueprints/Furniture/BP_A_CabinetDrawer` (`self.GetOwner`)))
      (bind _initems_2 (`/Game/Blueprints/Furniture/BP_A_Furniture.InItems` _asbp_a_cabinet_drawer_2))
      (if (`KismetArrayLibrary.Array_IsValidIndex` _initems_2)
        (for _array_element_2 _initems_2
          (`PrimitiveComponent.SetCollisionResponseToChannel` (`/Game/Blueprints/ItemInteractables/BP_A_ItemInteractable.Collision` _array_element_2) "ECC_Visibility" "ECR_Ignore"))))))

(event `OpenDrawer`
  (goto _label_2 :!via `PlayFromStart`))

(event `self.StaticMesh.OnClicked`
  (params (TouchedComponent :type "PrimitiveComponent Object Reference") (ButtonPressed :type "Key Structure"))
  (if (== (`self.GetOwner`) (`/Game/ThirdPerson/Blueprints/BP_ThirdPersonCharacter.CurrentFurniture` (`self.As BP Third Person Character`)))
    (if (`self.isOpen`)
      (`self.Close`)
      (else
        (`self.Open`)))))

(event `self.StaticMesh.OnBeginCursorOver`
  (params (TouchedComponent :type "PrimitiveComponent Object Reference"))
  (if (not (`self.isOpen`))
    (`PrimitiveComponent.SetMaterial` (`self.StaticMesh`) 0 "/Game/Blueprints/Materials/Highlight.Highlight")))

(event `self.StaticMesh.OnEndCursorOver`
  (params (TouchedComponent :type "PrimitiveComponent Object Reference"))
  (if (not (`self.isOpen`))
    (`PrimitiveComponent.SetMaterial` (`self.StaticMesh`) 0 null)))

(fn `Close`
  (set `self.isOpen` false)
  (`KismetSystemLibrary.PrintString` "Close")
  (for _array_element (`self.GetAttachedActors` true)
    (bind _asbp_a_grid (cast `/Game/Blueprints/Box/Grids/BP_A_Grid` _array_element))
    (`PrimitiveComponent.SetCollisionEnabled` (`/Game/Blueprints/Box/Grids/BP_A_Grid.Box` _asbp_a_grid) "NoCollision"))
  (`self.Closed`))

(fn `Open`
  (set `self.isOpen` true)
  (`KismetSystemLibrary.PrintString` "Open")
  (for _array_element (`self.GetAttachedActors` true)
    (bind _asbp_a_grid (cast `/Game/Blueprints/Box/Grids/BP_A_Grid` _array_element))
    (`PrimitiveComponent.SetCollisionEnabled` (`/Game/Blueprints/Box/Grids/BP_A_Grid.Box` _asbp_a_grid) "QueryOnly"))
  (`self.Opened`)
  (bind _asbp_a_cabinet_drawer (cast `/Game/Blueprints/Furniture/BP_A_CabinetDrawer` (`self.GetOwner`)))
  (for _array_element_2 (`/Game/Blueprints/Furniture/BP_A_Furniture.FurniturePartsChild` _asbp_a_cabinet_drawer)
    (if (!= _array_element_2 self)
      (bind _asbp_a_drawer (cast `/Game/Blueprints/Furniture/FurnitureParts/BP_A_Drawer` _array_element_2))
      (if (`/Game/Blueprints/Furniture/FurnitureParts/BP_A_Drawer.isOpen` _asbp_a_drawer)
        (`self.Close` _asbp_a_drawer)
        (`KismetSystemLibrary.PrintString` "Close"))))
  (`PrimitiveComponent.SetMaterial` (`self.StaticMesh`) 0 null))

(fn `UserConstructionScript`)