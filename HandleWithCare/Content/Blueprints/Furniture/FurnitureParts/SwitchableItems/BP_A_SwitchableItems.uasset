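; Switchable slot on a furniture piece that shows whether an item is fitted, using its static mesh as a stand-in.
; SwitchMesh sets the material; when filling, it parks the given item at a fixed point below the origin, or spawns the assigned class there.
; Clicking a filled slot returns the item to the furniture's initial location as draggable and restores the red highlight.
; Both paths update the owning furniture's InItems and OutItems lists.
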(event `self.ReceiveBeginPlay`
  (bind _asbp_third_person_character (cast `/Game/ThirdPerson/Blueprints/BP_ThirdPersonCharacter` (`GameplayStatics.GetPlayerPawn` 0)))
  (set `self.As BP Third Person Character` _asbp_third_person_character))

(event `self.StaticMesh.OnClicked`
  (params (TouchedComponent :type "PrimitiveComponent Object Reference") (ButtonPressed :type "Key Structure"))
  (bind _currentitem (`self.CurrentItem`))
  (bind _currentitem_2 (`self.CurrentItem`))
  (bind _marker (`self.Marker`))
  (if (`self.hasMesh`)
    (bind _asbp_a_furniture (cast `/Game/Blueprints/Furniture/BP_A_Furniture` (`self.GetOwner`)))
    (`/Engine/EditorBlueprintResources/StandardMacros.IsValid` _currentitem
      (:`Is Valid`
        (`self.K2_SetActorLocationAndRotation` _currentitem (`SceneComponent.K2_GetComponentLocation` (`/Game/Blueprints/Furniture/BP_A_Furniture.ItemInitialLocation` _asbp_a_furniture)) (`self.K2_GetActorRotation` _asbp_a_furniture) false false)
        (`KismetArrayLibrary.Array_AddUnique` (`/Game/Blueprints/Furniture/BP_A_Furniture.OutItems` _asbp_a_furniture) _currentitem)
        (`KismetArrayLibrary.Array_RemoveItem` (`/Game/Blueprints/Furniture/BP_A_Furniture.InItems` _asbp_a_furniture) _currentitem_2)
        (set `/Game/Blueprints/ItemInteractables/BP_A_ItemInteractable.canBeDragged` true _currentitem_2)
        (set `/Game/Blueprints/ItemInteractables/BP_A_ItemInteractable.isInMesh` false _currentitem_2)
        (set `/Game/Blueprints/ItemInteractables/BP_A_ItemInteractable.StackOwner` _currentitem_2 _currentitem_2)
        (set `self.CurrentItem` null)
        (`self.SwitchMesh` false null "/Game/Blueprints/Materials/HighlightRed.HighlightRed")
        (if (not (`SceneComponent.bHiddenInGame` _marker))
          (`SceneComponent.SetHiddenInGame` _marker true false))))))

(fn `SwitchMesh`
  (params (hasMesh :type Boolean) (Target :type "/Game/Blueprints/ItemInteractables/BP_A_ItemInteractable Object Reference") (Material :type "MaterialInterface Object Reference"))
  (`PrimitiveComponent.SetMaterial` (`self.StaticMesh`) 0 Material)
  (bind _output_get (set `self.hasMesh` hasMesh))
  (if _output_get
    (`PrimitiveComponent.SetCollisionResponseToChannel` (`self.StaticMesh`) "ECC_Visibility" "ECR_Block")
    (bind _asbp_a_furniture (cast `/Game/Blueprints/Furniture/BP_A_Furniture` (`self.GetOwner`)))
    (bind _output_get_2 (set `self.CurrentItem` Target))
    (`/Engine/EditorBlueprintResources/StandardMacros.IsValid` (`self.CurrentItem`)
      (:`Is Valid`
        (`/Engine/EditorBlueprintResources/StandardMacros.IsValid` Target
          (:`Is Valid`
            (`KismetArrayLibrary.Array_RemoveItem` (`/Game/Blueprints/Furniture/BP_A_Furniture.OutItems` _asbp_a_furniture) Target)
            (bind _initems (`/Game/Blueprints/Furniture/BP_A_Furniture.InItems` _asbp_a_furniture))
            (`KismetArrayLibrary.Array_AddUnique` _initems Target)
            (`self.K2_SetActorLocation` _output_get_2 (0.0 0.0 -50.0) false false)
            (set `/Game/Blueprints/ItemInteractables/BP_A_ItemInteractable.isInMesh` true _output_get_2))))
      (:`Is Not Valid`
        (bind _returnvalue (`|SpawnActorFromClass` (`self.ItemAssigned`) (`KismetMathLibrary.MakeTransform` (0.0 0.0 -50.0)) "Undefined" "MultiplyWithRoot" null null))
        (`KismetArrayLibrary.Array_AddUnique` _initems _returnvalue)
        (bind _output_get_3 (set `self.CurrentItem` _returnvalue))
        (set `/Game/Blueprints/ItemInteractables/BP_A_ItemInteractable.isInMesh` true _output_get_3)))
    (else
      (`PrimitiveComponent.SetMaterial` (`self.StaticMesh`) 0 "/Game/Blueprints/Materials/HighlightRed.HighlightRed"))))

(fn `UserConstructionScript`)