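; Player truck pawn for what appears to be a level-select map, where pressing E at the current objective's building opens its level, or Ending for one specific objective.
; Before loading, it saves the building's spawn location to the game instance.
; StartMoving nudges the truck toward the level-select objective through a delayed recursive loop, while Tick yaws a second mesh toward TargetObjective.
; Steering, driving, location restore, target lookup and widget logic are disconnected.
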(event `self.ReceiveBeginPlay`
  (bind _asbp_player_controller (cast `/Game/Blueprints/Player/BP_PlayerController` (`self.GetController`)))
  (set `self.As BP Player Controller` _asbp_player_controller)
  (`EnhancedInputSubsystemInterface.AddMappingContext` (pcsubsystem `EnhancedInputLocalPlayerSubsystem` _asbp_player_controller) "/Game/Blueprints/CarMovement/IMC_CarControl.IMC_CarControl" 0 (struct))
  (bind _asbp_game_instance (cast `/Game/GameInstance/BP_GameInstance` (`GameplayStatics.GetGameInstance`)))
  (set `self.As BP Game Instance` _asbp_game_instance))

(event `EnhancedInput|/Game/Blueprints/CarMovement/IA_Throttle`
  (params (ActionValue :type "Float (double-precision)") (ElapsedSeconds :type "Float (double-precision)") (TriggeredSeconds :type "Float (double-precision)") (InputAction :type "InputAction Object Reference" :default "/Game/Blueprints/CarMovement/IA_Throttle.IA_Throttle"))
  (:`Triggered`
    (set `self.isMoving` true))
  (:`Completed`
    (set `self.isMoving` false)))

(event `EnhancedInput|/Game/Blueprints/CarMovement/IA_Steer`
  (params (ActionValue :type "Float (double-precision)") (ElapsedSeconds :type "Float (double-precision)") (TriggeredSeconds :type "Float (double-precision)") (InputAction :type "InputAction Object Reference" :default "/Game/Blueprints/CarMovement/IA_Steer.IA_Steer")))

(event `self.ReceiveTick`
  (params (DeltaSeconds :type "Float (single-precision)"))
  (bind (_returnvalue_roll _returnvalue_pitch _returnvalue_yaw) (`KismetMathLibrary.BreakRotator` (`KismetMathLibrary.FindLookAtRotation` (`SceneComponent.K2_GetComponentLocation` (`self.StaticMesh`)) (`self.TargetObjective`))))
  (`SceneComponent.K2_SetWorldRotation` (`self.StaticMesh1`) (`KismetMathLibrary.MakeRotator` 0.0 0.0 _returnvalue_yaw) false false))

(event `Key|E`
  (params (Key :type "Key Structure"))
  (bind _currentbuilding (`self.CurrentBuilding`))
  (bind _as_bp_game_instance (`self.As BP Game Instance`))
  (bind _currentobjective (`/Game/GameInstance/BP_GameInstance.CurrentObjective` _as_bp_game_instance))
  (:`Pressed`
    (`/Engine/EditorBlueprintResources/StandardMacros.IsValid` _currentbuilding
      (:`Is Valid`
        (if (`|EnumEquality` (`/Game/LevelSelectTest/Actors/BP_BaseBuilding.QuestTrigger` _currentbuilding) _currentobjective)
          (setmembers `/Game/GameInstance/Structures/LocationData` :`StructRef` (`/Game/GameInstance/BP_GameInstance.LocationStruct` _as_bp_game_instance) :`LastKnownLocation` (`KismetMathLibrary.MakeTransform` (`SceneComponent.K2_GetComponentLocation` (`/Game/LevelSelectTest/Actors/BP_BaseBuilding.SpawnLocation` _currentbuilding))))
          (if (`|EnumEquality` _currentobjective "NewEnumerator12")
            (`GameplayStatics.OpenLevel` "Ending")
            (else
              (`GameplayStatics.OpenLevel` (`/Game/LevelSelectTest/Actors/BP_BaseBuilding.GoToLevel` _currentbuilding)))))))))

(event `StartMoving`
  (if (not (`self.Stop`))
    (bind _returnvalue (`GameplayStatics.GetActorOfClass` "/Game/LevelSelectTest/BP_A_LevelSelect_Objective.BP_A_LevelSelect_Objective_C"))
    (bind _returnvalue_2 (- (`self.K2_GetActorLocation` _returnvalue) (`self.K2_GetActorLocation`)))
    (`SceneComponent.K2_AddWorldOffset` (`self.StaticMesh`) (* (`KismetMathLibrary.Normal` _returnvalue_2) 3.0) false false)
    (if (not (< (`KismetMathLibrary.VSize` _returnvalue_2) 60.0))
      (`KismetSystemLibrary.Delay` 0.01)
      (`self.StartMoving`))))

(fn `UserConstructionScript`)