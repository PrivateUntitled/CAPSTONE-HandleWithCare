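; Office building actor on the level select map that configures itself as the Level 3 entry point.
; On BeginPlay, after the parent logic, it checks the game instance's current objective and sets level information, quest trigger and destination level when it matches.
; Nested within that match, it moves the level select truck to its spawn point, with an else branch meant to target the building for a following objective.
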(event `self.ReceiveBeginPlay`
  (bind _currentobjective (`/Game/GameInstance/BP_GameInstance.CurrentObjective` (`self.As BP Game Instance`)))
  (bind _returnvalue (`|EnumEquality` _currentobjective "NewEnumerator11"))
  (`parent.ReceiveBeginPlay`)
  (if _returnvalue
    (set `self.Level Information` "/Game/Blueprints/LevelSelect/Widgets/DA_Level3Information.DA_Level3Information")
    (set `self.QuestTrigger` "NewEnumerator11")
    (set `self.GoToLevel` "Level3")
    (if (or (`|EnumEquality` _currentobjective "NewEnumerator0") (`|EnumEquality` _currentobjective "NewEnumerator4") _returnvalue)
      (`self.K2_SetActorLocation` (`self.As BP Truck LS`) (`SceneComponent.K2_GetComponentLocation` (`self.SpawnLocation`)) false false)
      (elif (`|EnumEquality` (`/Game/GameInstance/BP_GameInstance.CurrentObjective` (`self.As BP Game Instance`)) "NewEnumerator12")
        (set `self.QuestTrigger` "NewEnumerator12")
        (set `/Game/Blueprints/CarMovement/BP_TruckLS.TargetObjective` (`self.K2_GetActorLocation`) (`self.As BP Truck LS`))))))

(fn `UserConstructionScript`
  (`parent.UserConstructionScript`))