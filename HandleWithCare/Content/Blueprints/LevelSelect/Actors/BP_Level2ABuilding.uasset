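; Level-select building actor for Level 2A that sets up the truck and the next quest target when the map starts.
; On BeginPlay, after the parent logic, it checks whether the game instance's current objective matches one specific stage.
; If it matches, it moves the level-select truck to its SpawnLocation, aims the truck's objective at the office building and assigns that stage as the office building's quest trigger.
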(event `self.ReceiveBeginPlay`
  (`parent.ReceiveBeginPlay`)
  (if (`|EnumEquality` (`/Game/GameInstance/BP_GameInstance.CurrentObjective` (`self.As BP Game Instance`)) "NewEnumerator14")
    (`self.K2_SetActorLocation` (`self.As BP Truck LS`) (`SceneComponent.K2_GetComponentLocation` (`self.SpawnLocation`)) false false)
    (bind _returnvalue (`GameplayStatics.GetActorOfClass` "/Game/Blueprints/LevelSelect/Actors/BP_OfficeBuilding.BP_OfficeBuilding_C"))
    (set `/Game/Blueprints/CarMovement/BP_TruckLS.TargetObjective` (`self.K2_GetActorLocation` _returnvalue) (`self.As BP Truck LS`))
    (set `/Game/Blueprints/LevelSelect/Actors/BP_BaseBuilding.QuestTrigger` "NewEnumerator14" _returnvalue)))

(fn `UserConstructionScript`
  (`parent.UserConstructionScript`))