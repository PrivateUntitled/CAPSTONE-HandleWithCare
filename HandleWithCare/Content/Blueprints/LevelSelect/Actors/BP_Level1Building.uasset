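; Level 1 building actor for the level select map, which can set where the truck starts.
; On BeginPlay it runs the parent logic, then checks the game instance's current objective against one specific enum value.
; On a match it moves the level select truck to the world location of its SpawnLocation component.
; The construction script only calls the parent.
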(event `self.ReceiveBeginPlay`
  (`parent.ReceiveBeginPlay`)
  (if (`|EnumEquality` (`/Game/GameInstance/BP_GameInstance.CurrentObjective` (`self.As BP Game Instance`)) "NewEnumerator10")
    (`self.K2_SetActorLocation` (`self.As BP Truck LS`) (`SceneComponent.K2_GetComponentLocation` (`self.SpawnLocation`)) false false)))

(fn `UserConstructionScript`
  (`parent.UserConstructionScript`))