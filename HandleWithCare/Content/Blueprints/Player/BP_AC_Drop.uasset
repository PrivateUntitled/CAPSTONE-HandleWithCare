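; Player component that drops carried items from BP_ThirdPersonCharacter back into the world as physics objects.
; Right mouse drops the last entry in Items when allowed, detaching it, enabling collision and physics, then recalculating weight and playing a sound.
; DropHoveredItem instead releases a specific item, freeing its grid cells, unlinking it from its stack and moving it to the current furniture's drop location, or to the player otherwise.
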(event `self.ReceiveBeginPlay`
  (bind _asbp_third_person_character (cast `/Game/ThirdPerson/Blueprints/BP_ThirdPersonCharacter` (`GameplayStatics.GetPlayerPawn` 0)))
  (set `self.As BP Third Person Character` _asbp_third_person_character))

(event `Key|RightMouseButton`
  (params (Key :type "Key Structure"))
  (bind _as_bp_third_person_character (`self.As BP Third Person Character`))
  (:`Pressed`
    (if (`/Game/ThirdPerson/Blueprints/BP_ThirdPersonCharacter.IsInteracting` _as_bp_third_person_character)
      _
      (elif (`/Game/ThirdPerson/Blueprints/BP_ThirdPersonCharacter.CanDrop` _as_bp_third_person_character)
        (`self.Dropitem`)))))

(event `Dropitem`
  (bind _items (`/Game/ThirdPerson/Blueprints/BP_ThirdPersonCharacter.Items` (`self.As BP Third Person Character`)))
  (bind _returnvalue (`KismetArrayLibrary.Array_LastIndex` _items))
  (bind _output (`|GetArrayItem` _items _returnvalue))
  (bind _collision (`/Game/Blueprints/ItemInteractables/BP_A_ItemInteractable.Collision` _output))
  (if (`KismetArrayLibrary.Array_IsValidIndex` (`/Game/ThirdPerson/Blueprints/BP_ThirdPersonCharacter.Items` (`self.As BP Third Person Character`)))
    (`PrimitiveComponent.SetConstraintMode` _collision "Default")
    (set `/Game/Blueprints/ItemInteractables/BP_A_ItemInteractable.canBeDragged` false _output)
    (`/Game/Blueprints/ItemInteractables/BP_A_ItemInteractable.ItemDropped` _output)
    (`Actor.K2_SetActorRotation` :`self` _output)
    (`Actor.K2_DetachFromActor` _output "KeepWorld" "KeepWorld" "KeepWorld")
    (`PrimitiveComponent.SetCollisionEnabled` _collision "QueryAndPhysics")
    (`PrimitiveComponent.SetCollisionResponseToChannel` _collision "ECC_Visibility" "ECR_Block")
    (`PrimitiveComponent.SetSimulatePhysics` _collision true)
    (`PrimitiveComponent.SetCollisionEnabled` (`/Game/Blueprints/ItemInteractables/BP_A_ItemInteractable.StaticMesh` _output) "PhysicsOnly")
    (`KismetArrayLibrary.Array_Remove` _items _returnvalue)
    (`KismetSystemLibrary.PrintString` "DRopped")
    (`/Game/ThirdPerson/Blueprints/BP_ThirdPersonCharacter.CalculateWeight` (`self.As BP Third Person Character`))
    (`GameplayStatics.PlaySound2D` "/Game/SOUND_DESIGN/SFX/SFX_Drop.SFX_Drop" 1.0 1.0 0.0 null null)))

(event `DropHoveredItem`
  (params (HoveredItem :type "/Game/Blueprints/ItemInteractables/BP_A_ItemInteractable Object Reference"))
  (bind _as_bp_third_person_character (`self.As BP Third Person Character`))
  (bind _gridused (`/Game/Blueprints/ItemInteractables/BP_A_ItemInteractable.GridUsed` HoveredItem))
  (bind _stackowner (`/Game/Blueprints/ItemInteractables/BP_A_ItemInteractable.StackOwner` HoveredItem))
  (bind _collision (`/Game/Blueprints/ItemInteractables/BP_A_ItemInteractable.Collision` HoveredItem))
  (bind _collision_2 (`/Game/Blueprints/ItemInteractables/BP_A_ItemInteractable.Collision` HoveredItem))
  (bind (_returnvalue_x _returnvalue_y _returnvalue_z) (`KismetMathLibrary.BreakVector` (`Actor.K2_GetActorLocation` _as_bp_third_person_character)))
  (bind _currentfurniture (`/Game/ThirdPerson/Blueprints/BP_ThirdPersonCharacter.CurrentFurniture` _as_bp_third_person_character))
  (if (`/Game/Blueprints/ItemInteractables/BP_A_ItemInteractable.isHolding` HoveredItem)
    _
    (elif (`/Game/ThirdPerson/Blueprints/BP_ThirdPersonCharacter.OnboardPackageUnpackDone` (`self.As BP Third Person Character`))
      (for _array_element _gridused
        (if (== _stackowner HoveredItem)
          (set `/Game/Blueprints/Box/Grids/BP_A_Grid.isOccupied` false _array_element)
          (`PrimitiveComponent.SetMaterial` (`/Game/Blueprints/Box/Grids/BP_A_Grid.Grid` _array_element) 0 "/Game/Textures/GridMaterial_InstGreen.GridMaterial_InstGreen")))
      (`KismetArrayLibrary.Array_Clear` _gridused)
      (if (not (== (`/Game/Blueprints/ItemInteractables/BP_A_ItemInteractable.StackOwner` HoveredItem) HoveredItem))
        (set `/Game/Blueprints/ItemInteractables/BP_A_ItemInteractable.PreviousStackOwner` _stackowner HoveredItem))
      (if (not (== _stackowner HoveredItem))
        (`KismetArrayLibrary.Array_RemoveItem` (`/Game/Blueprints/ItemInteractables/BP_A_ItemInteractable.ItemStack` _stackowner) HoveredItem))
      (`/Game/Blueprints/ItemInteractables/BP_A_ItemInteractable.RecalcualtePreviousStackOwner` HoveredItem)
      (`Actor.K2_DetachFromActor` HoveredItem "KeepWorld" "KeepWorld" "KeepWorld")
      (set `/Game/Blueprints/ItemInteractables/BP_A_ItemInteractable.canBeDragged` false HoveredItem)
      (set `/Game/Blueprints/ItemInteractables/BP_A_ItemInteractable.StackOwner` HoveredItem HoveredItem)
      (set `/Game/Blueprints/ItemInteractables/BP_A_ItemInteractable.canBeDragged` false HoveredItem)
      (`PrimitiveComponent.SetCollisionEnabled` _collision_2 "QueryAndPhysics")
      (`PrimitiveComponent.SetCollisionResponseToChannel` _collision_2 "ECC_Visibility" "ECR_Block")
      (`PrimitiveComponent.SetSimulatePhysics` _collision_2 true)
      (`KismetArrayLibrary.Array_RemoveItem` (`/Game/ThirdPerson/Blueprints/BP_ThirdPersonCharacter.Items` (`self.As BP Third Person Character`)) HoveredItem)
      (`/Engine/EditorBlueprintResources/StandardMacros.IsValid` _currentfurniture
        (:`Is Valid`
          (`Actor.K2_SetActorLocation` HoveredItem (`SceneComponent.K2_GetComponentLocation` (`/Game/Blueprints/Furniture/BP_A_Furniture.DropLocation` _currentfurniture)) false false)
          (`PrimitiveComponent.SetConstraintMode` _collision "Default"))
        (:`Is Not Valid`
          (`Actor.K2_SetActorLocation` HoveredItem (`KismetMathLibrary.MakeVector` _returnvalue_x _returnvalue_y (+ _returnvalue_z 10.0)) false false)
          (`PrimitiveComponent.SetConstraintMode` _collision "Default"))))))