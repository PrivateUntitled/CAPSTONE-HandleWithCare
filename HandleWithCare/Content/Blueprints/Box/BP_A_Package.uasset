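; BP_A_Package is an interactable cardboard box that the player picks up, or opens to pack and unpack items.
; Construction builds a grid of child cell actors, which BeginPlay can pre-populate with items.
; Pressing E while hovering switches the view to the box, hides surrounding clutter, lays out carried items and shows the box UI.
; Timelines swing the flaps and, once a stored box closes, lift, spin and shrink it away.
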(event `self.ReceiveBeginPlay`
  (bind _rightflap (`self.RightFlap`))
  (bind _leftflap (`self.LeftFlap`))
  (`parent.ReceiveBeginPlay`)
  (bind _asbp_gm_main (cast `/Game/Blueprints/GameModes/BP_GM_Main` (`GameplayStatics.GetGameMode`)))
  (set `self.As BP GM Main` _asbp_gm_main)
  (bind _returnvalue (`|GenericCreateObject` "/Game/Blueprints/Player/PlayerUI/WB_BoxUI.WB_BoxUI_C"))
  (set `self.BoxWidget` _returnvalue)
  (add `self.OnOpenPackage` (delegate `OnPackageOpened`))
  (add `self.OnClosePackage` (delegate `OnPackageClosed`))
  (`KismetArrayLibrary.Array_Add` (`self.MaterialStruct`) (make `/Game/Blueprints/Enums/StaticMeshStruct` _rightflap (`MeshComponent.GetMaterials` _rightflap)))
  (`KismetArrayLibrary.Array_Add` (`self.MaterialStruct`) (make `/Game/Blueprints/Enums/StaticMeshStruct` _leftflap (`MeshComponent.GetMaterials` _leftflap)))
  (`self.CalculatePackageWeight`)
  (if (`KismetArrayLibrary.Array_IsNotEmpty` (`self.ItemsToPopulate`))
    (`self.PopulateItems`)))

(event `OnPackageOpened`
  (bind (_returnvalue_roll _returnvalue_pitch _returnvalue_yaw) (`KismetMathLibrary.BreakRotator` (`self.K2_GetActorRotation`)))
  (bind (_returnvalue_x _returnvalue_y _returnvalue_z) (`KismetMathLibrary.BreakVector` (`self.K2_GetActorLocation`)))
  (`self.CheckSurroundingItems` true)
  (`|ExecutionSequence`
    (:`then_0`
      (bind (_direction _leftdooropen) (`Timeline|Timeline_3` :!via `PlayFromStart` :!label _label)
        (:`Update`
          (`SceneComponent.K2_SetRelativeRotation` (`self.LeftFlap`) (`KismetMathLibrary.MakeRotator` (`KismetMathLibrary.Lerp` (`self.LeftFlapCloseFloat`) (`self.LeftFlapOpenFloat`) _leftdooropen)) false false)
          (bind (_direction_2 _leftdooropen_2) (`Timeline|Timeline_1` :!via `Stop` :!label _label_2)
            (:`Update`
              (`SceneComponent.K2_SetRelativeRotation` (`self.LeftFlap`) (`KismetMathLibrary.MakeRotator` (`KismetMathLibrary.Lerp` (`self.LeftFlapOpenFloat`) (`self.LeftFlapCloseFloat`) _leftdooropen_2)) false false)
              (goto _label :!via `Stop`))
            (:`Finished`
              (if (`self.isStored`)
                (`self.Stored`)
                (bind (_direction_3 _upbox) (`Timeline|BoxAway` :!via `PlayFromStart`)
                  (:`Update`
                    (`self.K2_SetActorLocation` (`KismetMathLibrary.MakeVector` _returnvalue_x _returnvalue_y (`KismetMathLibrary.Lerp` _returnvalue_z (+ _returnvalue_z 2.0) _upbox))))
                  (:`Finished`
                    (`|ExecutionSequence`
                      (:`then_0`
                        (bind (_direction_4 _spin) (`Timeline|SpinBox` :!via `PlayFromStart`)
                          (:`Update`
                            (`self.K2_SetActorRotation` (`KismetMathLibrary.MakeRotator` 0.0 0.0 (+ _spin _returnvalue_yaw))))))
                      (:`then_1`
                        (`KismetSystemLibrary.K2_SetTimerDelegate` (delegate `PlayBoxScaleAnim`) 1.0)))))))))))
    (:`then_1`
      (bind (_direction_5 _rightdooropen) (`Timeline|Timeline_0` :!via `PlayFromStart` :!label _label_3)
        (:`Update`
          (`SceneComponent.K2_SetRelativeRotation` (`self.RightFlap`) (`KismetMathLibrary.MakeRotator` (`KismetMathLibrary.Lerp` (`self.RightFlapCloseFloat`) (`self.RightFlapOpenFloat`) _rightdooropen)) false false)
          (bind (_direction_6 _rightdooropen_2) (`Timeline|Timeline_2` :!via `Stop` :!label _label_4)
            (:`Update`
              (`SceneComponent.K2_SetRelativeRotation` (`self.RightFlap`) (`KismetMathLibrary.MakeRotator` (`KismetMathLibrary.Lerp` (`self.RightFlapOpenFloat`) (`self.RightFlapCloseFloat`) _rightdooropen_2)) false false)
              (goto _label_3 :!via `Stop`))))))))

(event `self.ReceiveActorBeginOverlap`
  (params (OtherActor :type "Actor Object Reference"))
  (`parent.ReceiveActorBeginOverlap` null))

(event `OnPackageClosed`
  (`self.CheckSurroundingItems` false "QueryOnly")
  (`|ExecutionSequence`
    (:`then_0`
      (goto _label_2 :!via `PlayFromStart`))
    (:`then_1`
      (goto _label_4 :!via `PlayFromStart`))))

(event `self.Collision.OnBeginCursorOver`
  (params (TouchedComponent :type "PrimitiveComponent Object Reference"))
  (bind _as_bp_third_person_character (`self.As BP Third Person Character`))
  (if (not (`/Game/ThirdPerson/Blueprints/BP_ThirdPersonCharacter.IsInteracting` _as_bp_third_person_character))
    (`self.On Hover`)
    (`self.EnableInput` (`/Game/ThirdPerson/Blueprints/BP_ThirdPersonCharacter.As BP Player Controller` _as_bp_third_person_character))))

(event `self.Collision.OnEndCursorOver`
  (params (TouchedComponent :type "PrimitiveComponent Object Reference"))
  (bind _as_bp_third_person_character (`self.As BP Third Person Character`))
  (if (not (`/Game/ThirdPerson/Blueprints/BP_ThirdPersonCharacter.IsInteracting` _as_bp_third_person_character))
    (`self.OnUnhover`)
    (`self.DisableInput` (`/Game/ThirdPerson/Blueprints/BP_ThirdPersonCharacter.As BP Player Controller` _as_bp_third_person_character))))

(event `self.Collision.OnClicked`
  (params (TouchedComponent :type "PrimitiveComponent Object Reference") (ButtonPressed :type "Key Structure"))
  (bind _as_bp_third_person_character (`self.As BP Third Person Character`))
  (if (`self.isInteracted`)
    _
    (elif (`/Game/ThirdPerson/Blueprints/BP_ThirdPersonCharacter.OnboardPackageUnpackDone` _as_bp_third_person_character)
      (`/Game/Blueprints/Player/BP_AC_PickUp.PickupItem` (`/Game/ThirdPerson/Blueprints/BP_ThirdPersonCharacter.BP_AC_PickUp` _as_bp_third_person_character)))))

(event `ShowOptions`)

(event `PlayBoxScaleAnim`
  (bind (_returnvalue_x _returnvalue_y _returnvalue_z) (`KismetMathLibrary.BreakVector` (`self.GetActorScale3D`)))
  (bind (_returnvalue_x_2 _returnvalue_y_2 _returnvalue_z_2) (`KismetMathLibrary.BreakVector` (`self.GetActorScale3D`)))
  (bind (_direction _scalebox) (`Timeline|BoxScaleBig` :!via `PlayFromStart`)
    (:`Update`
      (bind _returnvalue (`KismetMathLibrary.Lerp` _returnvalue_z_2 1.2 _scalebox))
      (`self.SetActorScale3D` (`KismetMathLibrary.MakeVector` _returnvalue _returnvalue _returnvalue)))
    (:`Finished`
      (bind (_direction_2 _scalebox_2) (`Timeline|BoxScaleSmall` :!via `PlayFromStart`)
        (:`Update`
          (bind _returnvalue_2 (`KismetMathLibrary.Lerp` _returnvalue_z 0.0 _scalebox_2))
          (`self.SetActorScale3D` (`KismetMathLibrary.MakeVector` _returnvalue_2 _returnvalue_2 _returnvalue_2)))
        (:`Finished`
          (`KismetSystemLibrary.PrintString` "Animation Closed done"))))))

(event `OpenBox`
  (bind _collision (`self.Collision`))
  (bind _as_bp_third_person_character (`self.As BP Third Person Character`))
  (bind _as_bp_third_person_character_2 (`self.As BP Third Person Character`))
  (bind _boxwidget (`self.BoxWidget`))
  (bind _items (`/Game/ThirdPerson/Blueprints/BP_ThirdPersonCharacter.Items` (`self.As BP Third Person Character`)))
  (`PlayerController.SetViewTargetWithBlend` (`/Game/ThirdPerson/Blueprints/BP_ThirdPersonCharacter.As BP Player Controller` _as_bp_third_person_character_2) self 0.0 "VTBlend_Linear" 0.0 false)
  (`PrimitiveComponent.SetSimulatePhysics` _collision false)
  (`PrimitiveComponent.SetCollisionEnabled` _collision "NoCollision")
  (`PrimitiveComponent.SetCollisionEnabled` (`self.StaticMesh`) "QueryAndPhysics")
  (`UserWidget.AddToViewport` (`self.BoxWidget`) 0)
  (`self.OnOpenPackage`)
  (`self.SetActorHiddenInGame` _as_bp_third_person_character_2 true)
  (`self.GetItems` (`self.ItemSpawnLocation`) _items)
  (for _array_element _items
    (set `/Game/Blueprints/ItemInteractables/BP_A_ItemInteractable.canBeDragged` true _array_element)
    (`PrimitiveComponent.SetCollisionResponseToChannel` (`/Game/Blueprints/ItemInteractables/BP_A_ItemInteractable.Collision` _array_element) "ECC_Visibility" "ECR_Block"))
  (set `self.OutBox` _items)
  (`KismetArrayLibrary.Array_Clear` _items)
  (set `/Game/ThirdPerson/Blueprints/BP_ThirdPersonCharacter.IsInteracting` true (`self.As BP Third Person Character`))
  (set `self.isInteracted` true)
  (for _array_element_2 (`self.InBox`)
    (`PrimitiveComponent.SetCollisionEnabled` (`/Game/Blueprints/ItemInteractables/BP_A_ItemInteractable.Collision` _array_element_2) "QueryAndPhysics"))
  (for _array_element_3 (`self.Grids_0`)
    (`/Engine/EditorBlueprintResources/StandardMacros.IsValid` _array_element_3
      (:`Is Valid`
        (bind _grid (`/Game/Blueprints/Box/Grids/BP_A_Grid.Grid` _array_element_3))
        (`SceneComponent.SetHiddenInGame` _grid false false)
        (`PrimitiveComponent.SetCollisionEnabled` (`/Game/Blueprints/Box/Grids/BP_A_Grid.Box` _array_element_3) "QueryOnly")
        (`PrimitiveComponent.SetCollisionResponseToChannel` _grid "ECC_Visibility" "ECR_Block"))))
  (`self.DisableInput` _as_bp_third_person_character (`/Game/ThirdPerson/Blueprints/BP_ThirdPersonCharacter.As BP Player Controller` _as_bp_third_person_character))
  (bind _outactors (`GameplayStatics.GetAllActorsOfClass` "BP_A_Package_C"))
  (for _array_element_4 _outactors
    (if (!= _array_element_4 self)
      (bind _collision_2 (`/Game/Blueprints/ItemInteractables/BP_A_ItemInteractable.Collision` _array_element_4))
      (`PrimitiveComponent.SetSimulatePhysics` _collision_2 false)
      (`PrimitiveComponent.SetCollisionEnabled` _collision_2 "NoCollision")
      (`PrimitiveComponent.SetCollisionEnabled` (`/Game/Blueprints/Box/BP_A_Package.Capsule` _array_element_4) "NoCollision")
      (`self.SetActorHiddenInGame` _array_element_4 true)
      (for _array_element_5 (`/Game/Blueprints/Box/BP_A_Package.InBox` _array_element_4)
        (`self.SetActorHiddenInGame` _array_element_5 true))))
  (bind _outactors_2 (`GameplayStatics.GetAllActorsOfClass` "/Game/Blueprints/Furniture/BP_A_Furniture.BP_A_Furniture_C"))
  (for _array_element_6 _outactors_2
    (`self.SetActorHiddenInGame` _array_element_6 true)
    (`self.SetActorEnableCollision` _array_element_6 false)
    (for _array_element_7 (`/Game/Blueprints/Furniture/BP_A_Furniture.InItems` _array_element_6)
      (`/Engine/EditorBlueprintResources/StandardMacros.IsValid` _array_element_7
        (:`Is Valid`
          (`self.SetActorHiddenInGame` _array_element_7 true)))))
  (`Widget.SetVisibility` (`/Game/Blueprints/Player/PlayerUI/WB_PlayerUI.WeightText` (`/Game/ThirdPerson/Blueprints/BP_ThirdPersonCharacter.PlayerUI` (`self.As BP Third Person Character`))) "Hidden")
  (if (`/Game/Blueprints/GameModes/BP_GM_Main.isPacking` (`self.As BP GM Main`))
    (`/Game/Blueprints/Player/PlayerUI/WB_BoxUI.SetPackAwayEnabled` _boxwidget "Visible" true)
    (else
      (`/Game/Blueprints/Player/PlayerUI/WB_BoxUI.SetPackAwayEnabled` _boxwidget "Hidden" false))))

(event `Key|E`
  (params (Key :type "Key Structure"))
  (bind _as_bp_third_person_character (`self.As BP Third Person Character`))
  (:`Pressed`
    (if (`/Game/ThirdPerson/Blueprints/BP_ThirdPersonCharacter.IsInteracting` _as_bp_third_person_character)
      _
      (elif (not (`KismetArrayLibrary.Array_Contains` (`/Game/ThirdPerson/Blueprints/BP_ThirdPersonCharacter.Items` (`self.As BP Third Person Character`)) self))
        (`self.OpenBox`)
        (`/Game/Blueprints/Player/BP_PlayerController.SetMouse` (`/Game/ThirdPerson/Blueprints/BP_ThirdPersonCharacter.As BP Player Controller` _as_bp_third_person_character) false true)
        (set `/Game/ThirdPerson/Blueprints/BP_ThirdPersonCharacter.CurrentBox` self _as_bp_third_person_character)
        (`KismetSystemLibrary.PrintString` "EEEEE")
        (`PrimitiveComponent.SetCollisionResponseToChannel` (`self.Box`) "ECC_Visibility" "ECR_Block")
        (`self.CalculatePackageWeight`)))))

(event `GetItems`
  (params (`Static Mesh Component` :type "StaticMeshComponent Object Reference") (Items :type "Array of /Game/Blueprints/ItemInteractables/BP_A_ItemInteractable Object Reference"))
  (for (_array_element _array_index) Items
    (if (== _array_index 0)
      (`self.K2_DetachFromActor` _array_element "KeepWorld" "KeepWorld" "KeepWorld")
      (`self.K2_SetActorLocation` _array_element (`SceneComponent.K2_GetComponentLocation` `Static Mesh Component`) false false)
      (`self.K2_SetActorRotation` _array_element (`KismetMathLibrary.ComposeRotators` (`SceneComponent.K2_GetComponentRotation` `Static Mesh Component`) (struct :`Yaw` 90.0)) false)
      (`self.PlayAssignedDialogue` _array_element)
      (else
        (bind _output (`|GetArrayItem` Items _array_index))
        (`self.K2_DetachFromActor` _output "KeepWorld" "KeepWorld" "KeepWorld")
        (bind (_origin _boxextent) (`KismetSystemLibrary.GetComponentBounds` (`/Game/Blueprints/ItemInteractables/BP_A_ItemInteractable.StaticMesh` (`|GetArrayItem` Items (- _array_index 1)))))
        (`self.K2_SetActorLocation` _output (`KismetMathLibrary.MakeVector` (.x _origin) (.y _origin) (+ (.z _origin) (* (.z _boxextent) 2.0))) false false)
        (`self.K2_SetActorRotation` _output (`KismetMathLibrary.ComposeRotators` (`SceneComponent.K2_GetComponentRotation` `Static Mesh Component`) (struct :`Yaw` 90.0)) false)
        (`self.PlayAssignedDialogue` _array_element)))))

(event `GetOutBoxItems`
  (bind _as_bp_third_person_character (`self.As BP Third Person Character`))
  (bind _outbox (`self.OutBox`))
  (bind _itemplacement (`/Game/ThirdPerson/Blueprints/BP_ThirdPersonCharacter.ItemPlacement` _as_bp_third_person_character))
  (`self.GetItems` _itemplacement _outbox)
  (for _array_element _outbox
    (set `/Game/Blueprints/ItemInteractables/BP_A_ItemInteractable.PreviousStackOwner` null _array_element)
    (`self.K2_AttachToComponent` _array_element _itemplacement "None" "KeepWorld" "KeepWorld" "KeepWorld" true)
    (bind _collision (`/Game/Blueprints/ItemInteractables/BP_A_ItemInteractable.Collision` _array_element))
    (`PrimitiveComponent.SetCollisionResponseToChannel` _collision "ECC_Visibility" "ECR_Ignore")
    (`PrimitiveComponent.SetCollisionEnabled` (`/Game/Blueprints/ItemInteractables/BP_A_ItemInteractable.StaticMesh` _array_element) "PhysicsOnly")
    (`PrimitiveComponent.SetConstraintMode` _collision "None"))
  (`PrimitiveComponent.SetCollisionResponseToChannel` (`self.Box`) "ECC_Visibility" "ECR_Ignore")
  (set `/Game/ThirdPerson/Blueprints/BP_ThirdPersonCharacter.Items` _outbox _as_bp_third_person_character)
  (`KismetArrayLibrary.Array_Clear` _outbox))

(event `DropOutBoxItems`
  (bind _outbox (`self.OutBox`))
  (bind (_returnvalue_x _returnvalue_y _returnvalue_z) (`KismetMathLibrary.BreakVector` (`self.K2_GetActorLocation` (`self.As BP Third Person Character`))))
  (for _array_element (`self.OutBox`)
    (set `/Game/Blueprints/ItemInteractables/BP_A_ItemInteractable.isPackaged` false _array_element)
    (set `/Game/Blueprints/ItemInteractables/BP_A_ItemInteractable.canBeDragged` false _array_element)
    (`self.K2_DetachFromActor` _array_element "KeepWorld" "KeepWorld" "KeepWorld")
    (bind _collision (`/Game/Blueprints/ItemInteractables/BP_A_ItemInteractable.Collision` _array_element))
    (`PrimitiveComponent.SetSimulatePhysics` _collision true)
    (`PrimitiveComponent.SetCollisionResponseToChannel` (`/Game/Blueprints/ItemInteractables/BP_A_ItemInteractable.Collision` _array_element) "ECC_Visibility" "ECR_Block")
    (`PrimitiveComponent.SetCollisionEnabled` (`/Game/Blueprints/ItemInteractables/BP_A_ItemInteractable.Collision` _array_element) "QueryAndPhysics")
    (`self.K2_SetActorLocation` _array_element (`KismetMathLibrary.MakeVector` _returnvalue_x _returnvalue_y (+ _returnvalue_z 10.0)) false false)
    (`PrimitiveComponent.SetConstraintMode` _collision "Default"))
  (for _array_element_2 _outbox
    (`KismetArrayLibrary.Array_RemoveItem` _outbox _array_element_2))
  (`PrimitiveComponent.SetCollisionResponseToChannel` (`self.Box`) "ECC_Visibility" "ECR_Ignore"))

(fn `CheckSurroundingItems`
  (params (bNewHidden :type Boolean) (NewType :type "ECollisionEnabled Enum" :default "NoCollision"))
  (for _array_element (`PrimitiveComponent.GetOverlappingActors` (`self.Capsule`) "/Game/Blueprints/ItemInteractables/BP_A_ItemInteractable.BP_A_ItemInteractable_C")
    (`KismetSystemLibrary.PrintString` (`KismetSystemLibrary.GetDisplayName` _array_element))
    (bind _asbp_a_item_interactable (cast `/Game/Blueprints/ItemInteractables/BP_A_ItemInteractable` _array_element))
    (if (`/Game/Blueprints/ItemInteractables/BP_A_ItemInteractable.canBeDragged` _asbp_a_item_interactable)
      _
      (elif (not (`KismetArrayLibrary.Array_Contains` (`/Game/ThirdPerson/Blueprints/BP_ThirdPersonCharacter.Items` (`self.As BP Third Person Character`)) _asbp_a_item_interactable))
        (`self.SetActorHiddenInGame` _array_element bNewHidden)))))

(fn `ClearGrid`
  (bind _grids_0 (`self.Grids_0`))
  (if (`KismetArrayLibrary.Array_IsValidIndex` (`self.Grids_0`))
    (bind (_arrayindex _arrayelement) (`/Engine/EditorBlueprintResources/StandardMacros.ReverseForEachLoop` _grids_0)
      (:`LoopBody`
        (`/Engine/EditorBlueprintResources/StandardMacros.IsValid` _arrayelement
          (:`Is Valid`
            (`self.K2_DestroyActor` _arrayelement))))
      (:`Completed`
        (`KismetArrayLibrary.Array_Clear` _grids_0)))))

(fn `InitializeGrid`
  (bind _gridlength (`self.GridLength`))
  (`self.ClearGrid`)
  (for _index (range (`self.Rows_0`))
    (for _index_2 (range (`self.Columns_0`))
      (bind _returnvalue (`AddComponent|NODE_AddChildActorComponent-0` :`RelativeTransform` (`KismetMathLibrary.MakeTransform` (`self.K2_GetActorLocation`) (`self.K2_GetActorRotation`))))
      (`ChildActorComponent.SetChildActorClass` _returnvalue "/Game/Blueprints/Box/Grids/BP_A_HorGrid.BP_A_HorGrid_C")
      (bind _asbp_a_grid (cast `/Game/Blueprints/Box/Grids/BP_A_Grid` (`ChildActorComponent.ChildActor` _returnvalue)))
      (`self.SetOwner` _asbp_a_grid self)
      (set `/Game/Blueprints/Box/Grids/BP_A_Grid.Row` _index _asbp_a_grid)
      (set `/Game/Blueprints/Box/Grids/BP_A_Grid.Column` _index_2 _asbp_a_grid)
      (set `/Game/Blueprints/Box/Grids/BP_A_Grid.GridCellSize` (`self.GridCellSize_0`) _asbp_a_grid)
      (bind _box (`/Game/Blueprints/Box/Grids/BP_A_Grid.Box` _asbp_a_grid))
      (`BoxComponent.SetBoxExtent` _box (`KismetMathLibrary.MakeVector` 40.0 40.0 _gridlength) true)
      (`SceneComponent.K2_SetRelativeLocation` _box (`KismetMathLibrary.MakeVector` 0.0 0.0 _gridlength) false false)
      (`/Game/Blueprints/Box/Grids/BP_A_Grid.Initialize` _asbp_a_grid (`self.GridAdjustor`))
      (`/Game/Blueprints/Box/Grids/BP_A_Grid.GetPositionXY` _asbp_a_grid)
      (`KismetArrayLibrary.Array_AddUnique` (`self.Grids_0`) _asbp_a_grid))))

(fn `PopulateItems`
  (if (`KismetArrayLibrary.Array_IsValidIndex` (`self.ItemsToPopulate`))
    (for _array_element (`self.ItemsToPopulate`)
      (for _array_element_2 (`/Game/Blueprints/DataAssets/PopulateItemsDataAssets/DA_PopulateItems.PopulateItemsStruct` _array_element)
        (`/Game/Blueprints/Player/BP_AC_PopulateItems.PopulateItems` (`self.BP_AC_PopulateItems`) (`self.Grids_0`) (break `/Game/Blueprints/Structure/PopulateItemsStruct` _array_element_2) (`.InitialColumn_12_08EABF644FC0E26138F02B9625A10D3A` (break `/Game/Blueprints/Structure/PopulateItemsStruct` _array_element_2)) (`.EndRow_14_7A8B15EE445E8A2B1BB91BA963DD0099` (break `/Game/Blueprints/Structure/PopulateItemsStruct` _array_element_2)) (`.EndColumn_16_2CEB51A9439026185000C7BC82E190C3` (break `/Game/Blueprints/Structure/PopulateItemsStruct` _array_element_2)) (`.Rotation_19_CBE0018B421A55AA5758EEA9B1EBAAAD` (break `/Game/Blueprints/Structure/PopulateItemsStruct` _array_element_2)) (`.Item_22_A1880C41486790E2DAEA9D81E4BCEC38` (break `/Game/Blueprints/Structure/PopulateItemsStruct` _array_element_2)) (`.NumberOfItems_25_21A11A934D797545D7F408A99A6CAEC9` (break `/Game/Blueprints/Structure/PopulateItemsStruct` _array_element_2)) self (`self.InBox`))))))

(fn `ShowGrid`)

(fn `UserConstructionScript`
  (`parent.UserConstructionScript`)
  (`self.InitializeGrid`))