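; Bedroom moving-box actor that starts play pre-filled with packaged items.
; On BeginPlay it runs the parent logic, calls PopulateItems, then flags every entry in InBox as packaged.
; Unconnected calls to the BPACPopulateItems component, which would lay out assorted books and shirts across grid cell ranges, remain in the graph but never run.
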(event `self.ReceiveBeginPlay`
  (`parent.ReceiveBeginPlay`)
  (`self.PopulateItems`)
  (for _array_element (`self.InBox`)
    (set `/Game/Blueprints/ItemInteractables/BP_A_ItemInteractable.isPackaged` true _array_element)))

(fn `UserConstructionScript`
  (`parent.UserConstructionScript`))