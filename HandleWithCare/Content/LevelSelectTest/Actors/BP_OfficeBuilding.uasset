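; BP_OfficeBuilding is an office building actor in the level select test area that ties the truck to the current objective.
; On BeginPlay it reads the objective from the game instance and, for two objective values, moves the level-select truck to its SpawnLocation component.
; For one other objective value, it sets its QuestTrigger to that objective and passes its own location to the truck as the target objective.
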(event `self.ReceiveBeginPlay`
  (bind _currentobjective (`/Game/GameInstance/BP_GameInstance.CurrentObjective` (`self.As BP Game Instance`)))
  (`parent.ReceiveBeginPlay`)
  (if (or (`|EnumEquality` _currentobjective "NewEnumerator0") (`|EnumEquality` _currentobjective "NewEnumerator4"))
    (`self.K2_SetActorLocation` (`self.As BP Truck LS`) (`SceneComponent.K2_GetComponentLocation` (`self.SpawnLocation`)) false false)
    (elif (`|EnumEquality` (`/Game/GameInstance/BP_GameInstance.CurrentObjective` (`self.As BP Game Instance`)) "NewEnumerator12")
      (set `self.QuestTrigger` "NewEnumerator12")
      (set `/Game/Blueprints/CarMovement/BP_TruckLS.TargetObjective` (`self.K2_GetActorLocation`) (`self.As BP Truck LS`)))))

(fn `UserConstructionScript`
  (`parent.UserConstructionScript`))